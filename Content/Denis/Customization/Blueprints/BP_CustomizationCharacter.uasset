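; Customizable character Blueprint with modular male and female body parts, hair and clothing.
; The construction script slaves hair, beard and clothing meshes to the main Mesh via master pose.
; It then registers each part in a male or female list on BPCustomizationComponent and passes Mesh as its base skeletal mesh.
; BeginPlay greatly enlarges the bounds scale of the hair and beard meshes, likely to avoid culling.
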(event `self.ReceiveBeginPlay`
  (`parent.ReceiveBeginPlay`)
  (`PrimitiveComponent.SetBoundsScale` (`self.Hair`) 1000.0)
  (`PrimitiveComponent.SetBoundsScale` (`self.Beard`) 1000.0)
  (`PrimitiveComponent.SetBoundsScale` (`self.FemaleHair`) 1000.0))

(fn `UserConstructionScript`
  (`parent.UserConstructionScript`)
  (`|ExecutionSequence`
    (:`then_0`
      (`SkinnedMeshComponent.SetLeaderPoseComponent` (`self.Hair`) (`self.Mesh`) false)
      (`SkinnedMeshComponent.SetLeaderPoseComponent` (`self.Beard`) (`self.Mesh`) false)
      (`SkinnedMeshComponent.SetLeaderPoseComponent` (`self.Pants`) (`self.Mesh`) false)
      (`SkinnedMeshComponent.SetLeaderPoseComponent` (`self.Shirt`) (`self.Mesh`) false)
      (`SkinnedMeshComponent.SetLeaderPoseComponent` (`self.Shoes`) (`self.Mesh`) false)
      (`SkinnedMeshComponent.SetLeaderPoseComponent` (`self.Tie`) (`self.Mesh`) false)
      (`SkinnedMeshComponent.SetLeaderPoseComponent` (`self.sneakers`) (`self.Mesh`) false)
      (`SkinnedMeshComponent.SetLeaderPoseComponent` (`self.FemaleHair`) (`self.Mesh`) false)
      (`SkinnedMeshComponent.SetLeaderPoseComponent` (`self.casualset`) (`self.Mesh`) false)
      (`SkinnedMeshComponent.SetLeaderPoseComponent` (`self.FemalePants`) (`self.Mesh`) false))
    (:`then_1`
      (`/Game/Denis/Customization/Components/BP_CustomizationComponent.AddMenActorComponent` (`self.BP_CustomizationComponent`) (`self.RightEye`))
      (`/Game/Denis/Customization/Components/BP_CustomizationComponent.AddMenActorComponent` (`self.BP_CustomizationComponent`) (`self.LeftEye`))
      (`/Game/Denis/Customization/Components/BP_CustomizationComponent.AddMenActorComponent` (`self.BP_CustomizationComponent`) (`self.brows`))
      (`/Game/Denis/Customization/Components/BP_CustomizationComponent.AddMenActorComponent` (`self.BP_CustomizationComponent`) (`self.eyelashes`))
      (`/Game/Denis/Customization/Components/BP_CustomizationComponent.AddMenActorComponent` (`self.BP_CustomizationComponent`) (`self.Hair`))
      (`/Game/Denis/Customization/Components/BP_CustomizationComponent.AddMenActorComponent` (`self.BP_CustomizationComponent`) (`self.Beard`))
      (`/Game/Denis/Customization/Components/BP_CustomizationComponent.AddMenActorComponent` (`self.BP_CustomizationComponent`) (`self.Shirt`))
      (`/Game/Denis/Customization/Components/BP_CustomizationComponent.AddMenActorComponent` (`self.BP_CustomizationComponent`) (`self.Pants`))
      (`/Game/Denis/Customization/Components/BP_CustomizationComponent.AddMenActorComponent` (`self.BP_CustomizationComponent`) (`self.Shoes`))
      (`/Game/Denis/Customization/Components/BP_CustomizationComponent.AddMenActorComponent` (`self.BP_CustomizationComponent`) (`self.Tie`))
      (`/Game/Denis/Customization/Components/BP_CustomizationComponent.AddFemaleActorComponent` (`self.BP_CustomizationComponent`) (`self.FemaleHair`))
      (`/Game/Denis/Customization/Components/BP_CustomizationComponent.AddFemaleActorComponent` (`self.BP_CustomizationComponent`) (`self.FemaleRightEye`))
      (`/Game/Denis/Customization/Components/BP_CustomizationComponent.AddFemaleActorComponent` (`self.BP_CustomizationComponent`) (`self.FemaleLeftEye`))
      (`/Game/Denis/Customization/Components/BP_CustomizationComponent.AddFemaleActorComponent` (`self.BP_CustomizationComponent`) (`self.Femaleeyelashes`))
      (`/Game/Denis/Customization/Components/BP_CustomizationComponent.AddFemaleActorComponent` (`self.BP_CustomizationComponent`) (`self.sneakers`))
      (`/Game/Denis/Customization/Components/BP_CustomizationComponent.AddFemaleActorComponent` (`self.BP_CustomizationComponent`) (`self.casualset`))
      (`/Game/Denis/Customization/Components/BP_CustomizationComponent.SetBaseSkeletalMeshComponent` (`self.BP_CustomizationComponent`) (`self.Mesh`))
      (`/Game/Denis/Customization/Components/BP_CustomizationComponent.AddFemaleActorComponent` (`self.BP_CustomizationComponent`) (`self.FemalePants`)))))