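; Actor component that applies and replicates each player's character customization: skeletal meshes, materials, morph targets and gender.
; On BeginPlay, non-dedicated authority loads settings from the GameInstance, while autonomous clients also send theirs to the server.
; ApplyCustomization matches mesh components by name, morphs CharacterMesh0 and toggles registered gender-specific components.
; OnReps reapply changes on clients, and autonomous clients refresh all players three times at one-second intervals.
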(event `self.ReceiveBeginPlay`
  (set `self.arrSkeletalMeshComponent` (`Actor.K2_GetComponentsByClass` (`self.GetOwner`) "/Script/Engine.SkeletalMeshComponent"))
  (if (`Actor.HasAuthority` (`self.GetOwner`))
    (if (not (`KismetSystemLibrary.IsDedicatedServer`))
      (bind (_morph _skeletalmesh _gender) (message `/Game/Denis/Customization/Components/Interface/BPI_CharacterSetting.GetCharacterSetting` (`GameplayStatics.GetGameInstance`)))
      (set `self.Morph` _morph)
      (set `self.Skeletal Mesh` _skeletalmesh)
      (set `self.Gender` _gender)
      (`self.RefrashEvent`))
    (elif (`|EnumEquality` (`Actor.GetLocalRole` (`self.GetOwner`)) "ROLE_AutonomousProxy")
      (bind (_morph_2 _skeletalmesh_2 _gender_2) (message `/Game/Denis/Customization/Components/Interface/BPI_CharacterSetting.GetCharacterSetting` (`GameplayStatics.GetGameInstance`)))
      (`self.ServerTransferCharacterSetting` _morph_2 _skeletalmesh_2 _gender_2)
      (`self.ApplyCustomization` (`self.arrSkeletalMeshComponent`) _morph_2 _skeletalmesh_2 _gender_2 "CharacterMesh0")
      (`KismetSystemLibrary.Delay` 1.0)
      (`self.Refresh All Player Data`)
      (`KismetSystemLibrary.Delay` 1.0)
      (`self.Refresh All Player Data`)
      (`KismetSystemLibrary.Delay` 1.0)
      (`self.Refresh All Player Data`))))

(event `ServerTransferCharacterSetting`
  (params (Morph :type "Array of /Game/Denis/Customization/Structure/FMorph Structure") (skeletalMesh :type "Array of /Game/Denis/Customization/Structure/FSkeletalMesh Structure") (Gender :type "/Game/Denis/Customization/Enum/Enum_CharacterGender Enum" :default "NewEnumerator0"))
  (set `self.Morph` Morph)
  (set `self.Skeletal Mesh` skeletalMesh)
  (set `self.Gender` Gender))

(event `self.ChangeAppearance`
  (params (morph :type "Array of /Game/Denis/Customization/Structure/FMorph Structure (by ref)") (skeletalMesh :type "Array of /Game/Denis/Customization/Structure/FSkeletalMesh Structure (by ref)") (Gender :type "/Game/Denis/Customization/Enum/Enum_CharacterGender Enum" :default "NewEnumerator0"))
  (`self.ApplyCustomization` (`self.arrSkeletalMeshComponent`) morph skeletalMesh Gender "CharacterMesh0"))

(event `self.SelectGender`
  (params (Gender :type "/Game/Denis/Customization/Enum/Enum_CharacterGender Enum" :default "NewEnumerator0"))
  (switch `/Game/Denis/Customization/Enum/Enum_CharacterGender` Gender
    (:`NewEnumerator0`
      (for _array_element (`self.menActorComponent`)
        (`SceneComponent.SetVisibility` _array_element true false)
        (`SceneComponent.SetVisibility` (`self.baseSkeletalMesh`) true false :!label _label))
      (for _array_element_2 (`self.femaleActorComponent`)
        (`SceneComponent.SetVisibility` _array_element_2 false false)
        (goto _label)))
    (:`NewEnumerator1`
      (for _array_element_3 (`self.menActorComponent`)
        (`SceneComponent.SetVisibility` _array_element_3 false false)
        (goto _label))
      (for _array_element_4 (`self.femaleActorComponent`)
        (`SceneComponent.SetVisibility` _array_element_4 true false)
        (goto _label)))))

(event `self.AddMenActorComponent`
  (params (MenComponent :type "SceneComponent Object Reference"))
  (`KismetArrayLibrary.Array_Add` (`self.menActorComponent`) MenComponent))

(event `self.AddFemaleActorComponent`
  (params (FemaleComponent :type "SceneComponent Object Reference"))
  (`KismetArrayLibrary.Array_Add` (`self.femaleActorComponent`) FemaleComponent))

(event `RefrashEvent`
  (`self.ApplyCustomization` (`self.arrSkeletalMeshComponent`) (`self.Morph`) (`self.Skeletal Mesh`) (`self.Gender`) "CharacterMesh0"))

(event `self.SetBaseSkeletalMeshComponent`
  (params (SkeletalMesh :type "SkeletalMeshComponent Object Reference"))
  (set `self.baseSkeletalMesh` SkeletalMesh))

(event `/Game/Main/Blueprints/MainProjectPart/Services/BPI_ServerDataRecipient.ServerUpdateData`
  (`self.RefreshAllPlayerDataEvent`))

(event `RefreshAllPlayerDataEvent`
  (`self.Refresh All Player Data`))

(fn `ApplyCustomization`
  (params (skeletalMeshComponent :type "Array of SkeletalMeshComponent Object Reference") (morph :type "Array of /Game/Denis/Customization/Structure/FMorph Structure") (skeletalMesh :type "Array of /Game/Denis/Customization/Structure/FSkeletalMesh Structure") (gender :type "/Game/Denis/Customization/Enum/Enum_CharacterGender Enum" :default "NewEnumerator0") (nameBaseSkeletalMesh :type String))
  (locals (localNameBaseSkeletalMesh :type String :default "CharacterMesh0") (localBaseSkeletalMesh :type "SkeletalMeshComponent Object Reference"))
  (set `local.localNameBaseSkeletalMesh` nameBaseSkeletalMesh)
  (for _array_element skeletalMeshComponent
    (bind _returnvalue (`KismetSystemLibrary.GetObjectName` _array_element))
    (if (`KismetStringLibrary.EqualEqual_StrStr` _returnvalue (`local.localNameBaseSkeletalMesh`))
      (set `local.localBaseSkeletalMesh` _array_element))
    (for _array_element_2 skeletalMesh
      (bind (_nameclass _nameitem _image _skeletalmesh _materials) (break `/Game/Denis/Customization/Structure/FSkeletalMesh` _array_element_2))
      (if (`KismetStringLibrary.EqualEqual_StrStr` _returnvalue _nameclass)
        (`SkinnedMeshComponent.SetSkinnedAssetAndUpdate` _array_element _skeletalmesh true)
        (for (_array_element_3 _array_index) _materials
          (`PrimitiveComponent.SetMaterial` _array_element _array_index _array_element_3)))))
  (for _array_element_4 morph
    (bind (_namemorph _value) (break `/Game/Denis/Customization/Structure/FMorph` _array_element_4))
    (for _array_element_5 _namemorph
      (`SkeletalMeshComponent.SetMorphTarget` (`local.localBaseSkeletalMesh`) (`KismetStringLibrary.Conv_StringToName` _array_element_5) _value false)))
  (`self.SelectGender` gender))

(fn `OnRep_Gender`
  (if (not (`Actor.HasAuthority` (`self.GetOwner`)))
    (`self.ApplyCustomization` (`self.arrSkeletalMeshComponent`) (`self.Morph`) (`self.Skeletal Mesh`) (`self.Gender`) "CharacterMesh0")
    (`KismetSystemLibrary.PrintString` "Установил кастомайз")))

(fn `OnRep_Morph`
  (if (not (`Actor.HasAuthority` (`self.GetOwner`)))
    (`self.ApplyCustomization` (`self.arrSkeletalMeshComponent`) (`self.Morph`) (`self.Skeletal Mesh`) (`self.Gender`) "CharacterMesh0")
    (`KismetSystemLibrary.PrintString` "Установил кастомайз")))

(fn `OnRep_Skeletal Mesh`
  (if (not (`Actor.HasAuthority` (`self.GetOwner`)))
    (`self.ApplyCustomization` (`self.arrSkeletalMeshComponent`) (`self.Morph`) (`self.Skeletal Mesh`) (`self.Gender`) "CharacterMesh0")
    (`KismetSystemLibrary.PrintString` "Установил кастомайз")))

(fn `Refresh All Player Data`
  (for _array_element (`GameStateBase.PlayerArray` (`GameplayStatics.GetGameState`))
    (bind _returnvalue (`Actor.GetComponentByClass` (`PlayerState.PawnPrivate` _array_element) "BP_CustomizationComponent_C"))
    (`/Engine/EditorBlueprintResources/StandardMacros.IsValid` _returnvalue
      (:`Is Valid`
        (`self.RefrashEvent` _returnvalue)))))