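; Actor component that keeps the player's first- or third-person view mode in the Game Instance and restores it on begin play.
; On non-authority instances only, it binds to the owner's BP_ViewModeComponent change event and writes each new mode to the Game Instance.
; After a one-second delay it reads the stored mode and applies it through that component.
; A separate GetViewMode function always returns first person.
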(event `self.ReceiveBeginPlay`
  (bind _returnvalue (`self.GetOwner`))
  (bind _returnvalue_2 (`Actor.GetComponentByClass` _returnvalue "/Game/Main/Blueprints/PlayerComponents/Camera/BP_ViewModeComponent.BP_ViewModeComponent_C"))
  (if (not (`Actor.HasAuthority` _returnvalue))
    (add `/Game/Main/Blueprints/PlayerComponents/Camera/BP_ViewModeComponent.OnChangeViewMode` _returnvalue_2 (delegate `OnChangeViewModeEvent`))
    (`KismetSystemLibrary.Delay` 1.0)
    (bind _viewmode (message `/Game/Main/Blueprints/PlayerComponents/Camera/BPI_ViewMode.GetViewMode` (`GameplayStatics.GetGameInstance`)))
    (`/Game/Main/Blueprints/PlayerComponents/Camera/BP_ViewModeComponent.ApplyViewMode` _returnvalue_2 _viewmode)))

(event `OnChangeViewModeEvent`
  (params (viewMode :type "/Game/Main/Blueprints/PlayerComponents/Camera/Enum/E_ViewMode Enum" :default "NewEnumerator0"))
  (switch `/Game/Main/Blueprints/PlayerComponents/Camera/Enum/E_ViewMode` viewMode
    (:`NewEnumerator0`
      _)
    (:`NewEnumerator1`
      _))
  (message `/Game/Main/Blueprints/PlayerComponents/Camera/BPI_ViewMode.SetViewMode` (`GameplayStatics.GetGameInstance`) viewMode))

(fn `GetViewMode`
  (returns (viewMode :type "/Game/Main/Blueprints/PlayerComponents/Camera/Enum/E_ViewMode Enum"))
  (return "NewEnumerator0"))