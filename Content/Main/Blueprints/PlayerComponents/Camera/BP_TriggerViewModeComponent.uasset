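; BP_TriggerViewModeComponent turns its owner's box into a trigger zone that switches the camera vantage point used by overlapping actors.
; On BeginPlay, only where the owner lacks authority, it binds to the first BoxComponent's begin and end overlap events.
; Entering actors with a BP_ViewModeComponent receive IdVantagePointActor; exiting ones receive OldIdVantagePointActor, a separate variable never captured here.
; Both transitions print a debug message.
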(event `self.ReceiveBeginPlay`
  (if (not (`Actor.HasAuthority` (`self.GetOwner`)))
    (bind _output_get (set `self.trigger` (`Actor.GetComponentByClass` (`self.GetOwner`) "/Script/Engine.BoxComponent")))
    (add `PrimitiveComponent.OnComponentBeginOverlap` _output_get (delegate `BeginEvent`))
    (add `PrimitiveComponent.OnComponentEndOverlap` _output_get (delegate `EndEvent`))))

(event `EndEvent`
  (params (OverlappedComponent :type "PrimitiveComponent Object Reference") (OtherActor :type "Actor Object Reference") (OtherComp :type "PrimitiveComponent Object Reference") (OtherBodyIndex :type Integer))
  (bind _returnvalue (`Actor.GetComponentByClass` OtherActor "/Game/Main/Blueprints/PlayerComponents/Camera/BP_ViewModeComponent.BP_ViewModeComponent_C"))
  (bind _oldidvantagepointactor (`self.oldIdVantagePointActor`))
  (`/Engine/EditorBlueprintResources/StandardMacros.IsValid` _returnvalue
    (:`Is Valid`
      (`/Game/Main/Blueprints/PlayerComponents/Camera/BP_ViewModeComponent.SetUseIdVantagePointActor` _returnvalue _oldidvantagepointactor)
      (`KismetSystemLibrary.PrintString` (`KismetStringLibrary.Concat_StrStr` "Trigger View точка в зоне " (`KismetStringLibrary.Conv_IntToString` _oldidvantagepointactor)) true true (struct :`R` 1.0 :`G` 0.875658 :`A` 1.0)))))

(event `BeginEvent`
  (params (OverlappedComponent :type "PrimitiveComponent Object Reference") (OtherActor :type "Actor Object Reference") (OtherComp :type "PrimitiveComponent Object Reference") (OtherBodyIndex :type Integer) (bFromSweep :type Boolean) (SweepResult :type "HitResult Structure (by ref)"))
  (bind _returnvalue (`Actor.GetComponentByClass` OtherActor "/Game/Main/Blueprints/PlayerComponents/Camera/BP_ViewModeComponent.BP_ViewModeComponent_C"))
  (`/Engine/EditorBlueprintResources/StandardMacros.IsValid` _returnvalue
    (:`Is Valid`
      (`/Game/Main/Blueprints/PlayerComponents/Camera/BP_ViewModeComponent.SetUseIdVantagePointActor` _returnvalue (`self.idVantagePointActor`))
      (`KismetSystemLibrary.PrintString` (`KismetStringLibrary.Concat_StrStr` "Trigger View точка в зоне" (`KismetStringLibrary.Conv_IntToString` (`self.idVantagePointActor`))) true true (struct :`G` 1.0 :`B` 0.17999 :`A` 1.0)))))