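; Player component for an ALS character that switches the camera between first person, third person and registered vantage point actors.
; First and third person set the ALS view mode, blend back to the owner, save the mode and fire a change notification.
; Vantage points blend the controller's view target to an indexed actor unless locked.
; They leave the saved mode untouched, so ResetViewMode restores the last character view.
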(event `self.ReceiveBeginPlay`
  (`self.Initialize`))

(event `ApplyThridPercon`
  (set `self.viewMode` "NewEnumerator1")
  (`ALSBaseCharacter.SetViewMode` (`self.As ALS Character BP`) "ThirdPerson" false)
  (`self.StopWatchingVantagePoint`)
  (bind _output_get (set `self.savedViewMode` "NewEnumerator1"))
  (`self.OnChangeViewMode` _output_get))

(event `ApplyFirstPerson`
  (set `self.viewMode` "NewEnumerator0")
  (`ALSBaseCharacter.SetViewMode` (`self.As ALS Character BP`) "FirstPerson" false)
  (`self.StopWatchingVantagePoint`)
  (bind _output_get (set `self.savedViewMode` "NewEnumerator0"))
  (`self.OnChangeViewMode` _output_get))

(event `ApplyCurrentVantagePoint`
  (params (idVantagePointActor :type Integer))
  (bind _output_get (set `self.idVantagePointActor` idVantagePointActor))
  (if (not (`self.lockVantagePoint`))
    (set `self.viewMode` "NewEnumerator2")
    (`PlayerController.SetViewTargetWithBlend` (`self.As ALS Player Controller`) (`|GetArrayItem` (`self.vantagePointActorList`) _output_get) 0.3 "VTBlend_Linear" 0.0 false)))

(event `ResetViewMode`
  (switch `/Game/Main/Blueprints/PlayerComponents/Camera/Enum/E_ViewMode` (`self.savedViewMode`)
    (:`NewEnumerator0`
      (`self.ApplyFirstPerson`))
    (:`NewEnumerator1`
      (`self.ApplyThridPercon`))
    (:`NewEnumerator2`
      (`self.ApplyCurrentVantagePoint` (`self.idVantagePointActor`)))))

(event `SetRightShoulder`
  (params (value :type Boolean))
  (`ALSBaseCharacter.SetRightShoulder` (`self.As ALS Character BP`) value))

(event `SetLockVantagePoint`
  (params (value :type Boolean))
  (set `self.lockVantagePoint` value))

(event `ApplyVantagePoint`
  (`self.ApplyCurrentVantagePoint` (`self.idVantagePointActor`)))

(event `ApplyViewMode`
  (params (viewMode :type "/Game/Main/Blueprints/PlayerComponents/Camera/Enum/E_ViewMode Enum" :default "NewEnumerator0"))
  (bind _output_get (set `self.viewMode` viewMode))
  (switch `/Game/Main/Blueprints/PlayerComponents/Camera/Enum/E_ViewMode` _output_get
    (:`NewEnumerator0`
      (`self.ApplyFirstPerson`))
    (:`NewEnumerator1`
      (`self.ApplyThridPercon`))))

(fn `AddVantagePointActor`
  (params (vantagePointActor :type "Actor Object Reference (by ref)"))
  (`KismetArrayLibrary.Array_Add` (`self.vantagePointActorList`) vantagePointActor))

(fn `Initialize`
  (bind _asals_character_bp (cast `/ALSV4_CPP/AdvancedLocomotionV4/Blueprints/CharacterLogic/ALS_CharacterBP` (`self.GetOwner`)))
  (set `self.As ALS Character BP` _asals_character_bp)
  (bind _asals_player_controller (cast `/ALSV4_CPP/AdvancedLocomotionV4/Blueprints/CharacterLogic/ALS_Player_Controller` (`Pawn.GetController` (`self.As ALS Character BP`))))
  (bind _output_get (set `self.As ALS Player Controller` _asals_player_controller))
  (set `self.Player Camera Manager` (`PlayerController.PlayerCameraManager` _output_get))
  (set `self.idVantagePointActor` 0))

(fn `LookAtCurrentVantagePoint`
  (params (point :type "Actor Object Reference"))
  (`PlayerController.SetViewTargetWithBlend` (`self.As ALS Player Controller`) point 0.3 "VTBlend_Linear" 0.0 false))

(fn `SetUseIdVantagePointActor`
  (params (idVantagePointActor :type Integer))
  (locals (id :type Integer))
  (`KismetSystemLibrary.PrintString` (`KismetStringLibrary.Concat_StrStr` "Задал точку смотрения ID: " (`KismetStringLibrary.Conv_IntToString` idVantagePointActor)))
  (bind _output_get (set `local.id` idVantagePointActor))
  (if (< _output_get (`KismetArrayLibrary.Array_Length` (`self.vantagePointActorList`)))
    (if (>= (`local.id`) 0)
      (bind _output_get_2 (set `self.idVantagePointActor` (`local.id`)))
      (`KismetSystemLibrary.PrintString` (`KismetStringLibrary.Concat_StrStr` "Задал точку смотрения: " (`KismetStringLibrary.Conv_IntToString` _output_get_2)))
      (else
        (set `self.idVantagePointActor` 0)))
    (else
      (set `self.idVantagePointActor` 0))))

(fn `StopWatchingVantagePoint`
  (bind _as_als_player_controller (`self.As ALS Player Controller`))
  (if (`KismetSystemLibrary.IsValid` _as_als_player_controller)
    (`PlayerController.SetViewTargetWithBlend` _as_als_player_controller (`self.GetOwner`) 0.3 "VTBlend_Linear" 0.0 false)))