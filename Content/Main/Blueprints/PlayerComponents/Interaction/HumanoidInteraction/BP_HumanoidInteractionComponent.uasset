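; Base component for paired humanoid interactions, tracking a partner, availability and invite state, with overridable hit and start/stop hooks.
; On authority, it watches the owner's first two box components and marks interaction available when both register the same actor implementing BPI_HumanoidInteraction.
; StartIteraction disables mantling and locks the view's vantage point; StopIteraction reverses this.
; The Start and Stop events call these functions inversely.
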(event `self.ReceiveBeginPlay`
  (bind _returnvalue (`Actor.K2_GetComponentsByClass` (`self.GetOwner`) "/Script/Engine.BoxComponent"))
  (if (`Actor.HasAuthority` (`self.GetOwner`))
    (set `self.descriptorA` (`|GetArrayItem` _returnvalue))
    (set `self.descriptorB` (`|GetArrayItem` _returnvalue 1))
    (add `PrimitiveComponent.OnComponentBeginOverlap` (`self.descriptorA`) (delegate `BeginEvent`))
    (add `PrimitiveComponent.OnComponentEndOverlap` (`self.descriptorA`) (delegate `EndEvent`))
    (add `PrimitiveComponent.OnComponentBeginOverlap` (`self.descriptorB`) (delegate `BeginEvent_2`))
    (add `PrimitiveComponent.OnComponentEndOverlap` (`self.descriptorB`) (delegate `EndEvent_2`))))

(event `BeginEvent`
  (params (OverlappedComponent :type "PrimitiveComponent Object Reference") (OtherActor :type "Actor Object Reference") (OtherComp :type "PrimitiveComponent Object Reference") (OtherBodyIndex :type Integer) (bFromSweep :type Boolean) (SweepResult :type "HitResult Structure (by ref)"))
  (if (`self.CheckActorbyValid` OtherActor)
    (set `self.descriptorActorA` OtherActor)
    (`self.CheckValidDescripterEvent`)))

(event `EndEvent`
  (params (OverlappedComponent :type "PrimitiveComponent Object Reference") (OtherActor :type "Actor Object Reference") (OtherComp :type "PrimitiveComponent Object Reference") (OtherBodyIndex :type Integer))
  (if (`self.CheckActorbyValid` OtherActor)
    (`self.NoHitEvent` (`self.descriptorActorA`))
    (set `self.descriptorActorA` null)))

(event `BeginEvent_2`
  (params (OverlappedComponent :type "PrimitiveComponent Object Reference") (OtherActor :type "Actor Object Reference") (OtherComp :type "PrimitiveComponent Object Reference") (OtherBodyIndex :type Integer) (bFromSweep :type Boolean) (SweepResult :type "HitResult Structure (by ref)"))
  (if (`self.CheckActorbyValid` OtherActor)
    (set `self.descriptorActorB` OtherActor)
    (`self.CheckValidDescripterEvent`)))

(event `EndEvent_2`
  (params (OverlappedComponent :type "PrimitiveComponent Object Reference") (OtherActor :type "Actor Object Reference") (OtherComp :type "PrimitiveComponent Object Reference") (OtherBodyIndex :type Integer))
  (if (`self.CheckActorbyValid` OtherActor)
    (`self.NoHitEvent` (`self.descriptorActorB`))
    (set `self.descriptorActorB` null)))

(event `CheckValidDescripterEvent`
  (bind _descriptoractora (`self.descriptorActorA`))
  (if (`self.CheckDescriptors`)
    (set `self.isAvailable` true)
    (if (`KismetSystemLibrary.IsValid` _descriptoractora)
      (bind _output_get (set `self.partner` _descriptoractora))
      (`self.PartherHitEvent` _output_get)
      (else
        (`KismetSystemLibrary.PrintString` "Невалиден" true true (struct :`R` 1.0 :`B` 0.198472 :`A` 1.0))))
    (else
      (set `self.isAvailable` false))))

(event `/Game/Main/Blueprints/PlayerComponents/Interaction/HumanoidInteraction/BPI_HumanoidInteraction.Stop`
  (`self.StartIteraction`))

(event `/Game/Main/Blueprints/PlayerComponents/Interaction/HumanoidInteraction/BPI_HumanoidInteraction.Start`
  (`self.StopIteraction`))

(event `PartherHitEvent`
  (params (partner :type "Actor Object Reference")))

(event `NoHitEvent`
  (params (partner :type "Actor Object Reference")))

(event `/Game/Main/Blueprints/PlayerComponents/Interaction/HumanoidInteraction/BPI_HumanoidInteraction.SetActivePartnerAction`
  (params (actor :type "Actor Object Reference"))
  (set `self.activePartner` actor))

(event `/Game/Main/Blueprints/PlayerComponents/Interaction/HumanoidInteraction/BPI_HumanoidInteraction.AllowAction`
  (`KismetSystemLibrary.PrintString` "allow"))

(event `/Game/Main/Blueprints/PlayerComponents/Interaction/HumanoidInteraction/BPI_HumanoidInteraction.SetInviteStage`
  (params (value :type Boolean))
  (bind _output_get (set `self.invite` value))
  (`self.ServerInvite` _output_get))

(event `ServerInvite`
  (params (value :type Boolean))
  (set `self.invite` value))

(fn `CheckActorbyValid`
  (params (inActor :type "Actor Object Reference"))
  (returns (result :type Boolean))
  (if (> (`KismetArrayLibrary.Array_Length` (`Actor.GetComponentsByInterface` inActor "/Game/Main/Blueprints/PlayerComponents/Interaction/HumanoidInteraction/BPI_HumanoidInteraction.BPI_HumanoidInteraction_C")) 0)
    (return true)
    (else
      (return false))))

(fn `CheckAvalibleDoing`
  (returns (value :type Boolean))
  (if (== (`self.isAvailable`) true)
    (if (== (`self.partnerIsAvalible`) true)
      (set `self.isAvalibleDoing` true)
      (return (`self.isAvalibleDoing`))
      (else
        _)))
  (set `self.isAvalibleDoing` false)
  (return false))

(fn `CheckDescriptors`
  (returns (isSuccess :type Boolean))
  (return (== (`self.descriptorActorA`) (`self.descriptorActorB`))))

(fn `GetInviteStage`
  (returns (value :type Boolean))
  (return (`self.invite`)))

(fn `GetNameHumanoidInteraction`
  (returns (Name :type String))
  (return (`self.name`)))

(fn `isAvailableStage`
  (returns (value :type Boolean))
  (return (`self.isAvailable`)))

(fn `IsAvalibleDoingStage`
  (returns (result :type Boolean))
  (return (`self.CheckAvalibleDoing`)))

(fn `IsProcessStage`
  (returns (value :type Boolean))
  (return (`self.isProcess`)))

(fn `SetActivePartnerForPartner`
  (params (actor :type "Actor Object Reference"))
  (bind _returnvalue (`Actor.GetComponentsByInterface` actor "/Game/Main/Blueprints/PlayerComponents/Interaction/HumanoidInteraction/BPI_HumanoidInteraction.BPI_HumanoidInteraction_C"))
  (bind _returnvalue_2 (`self.GetOwner` self))
  (`KismetSystemLibrary.PrintString` (`KismetStringLibrary.Conv_IntToString` (`KismetArrayLibrary.Array_Length` _returnvalue)) true true (struct :`R` 1.0 :`B` 0.198472 :`A` 1.0))
  (for _array_element _returnvalue
    (message `/Game/Main/Blueprints/PlayerComponents/Interaction/HumanoidInteraction/BPI_HumanoidInteraction.SetActivePartnerAction` _array_element _returnvalue_2)
    (`KismetSystemLibrary.PrintString` (`KismetStringLibrary.Concat_StrStr` "activePartner " (`KismetSystemLibrary.GetDisplayName` _returnvalue_2)))))

(fn `SetActivityMantleComponent`
  (params (value :type Boolean))
  (message `/Game/Main/Blueprints/PlayerComponents/Player/Interface/BPI_ControlMantle.SetActivityMantle` (`|GetArrayItem` (`Actor.GetComponentsByInterface` (`self.GetOwner`) "/Game/Main/Blueprints/PlayerComponents/Player/Interface/BPI_ControlMantle.BPI_ControlMantle_C")) value))

(fn `SetLockVantagePoint`
  (params (value :type Boolean))
  (`/Game/Main/Blueprints/PlayerComponents/Camera/BP_ViewModeComponent.SetLockVantagePoint` (`Actor.GetComponentByClass` (`self.GetOwner`) "/Game/Main/Blueprints/PlayerComponents/Camera/BP_ViewModeComponent.BP_ViewModeComponent_C") value))

(fn `StartIteraction`
  ;[1 1 1] Вирутальный метод
  (set `self.isProcess` true)
  (set `self.isWorking` true)
  (`self.SetActivityMantleComponent` false)
  (`self.SetLockVantagePoint` true))

(fn `StopIteraction`
  (set `self.isProcess` false)
  (set `self.isWorking` false)
  (`self.SetActivityMantleComponent` true)
  (`self.SetLockVantagePoint` false))