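; Humanoid interaction component that lets two ALS characters perform a high five.
; A None/Waiting/Action status drives overlay states and replicated montages, relayed through server and client events.
; A waiting player invites a partner who enters the zone via a HUD message; acceptance routes back through the server to trigger the action.
; The action sets the partner on a scene slot, locks both characters' input while they animate, then stops and resets.
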(event `self.ReceiveBeginPlay`
  (`parent.ReceiveBeginPlay`)
  (`self.Initialize`)
  (set `self.viewMode` (`Actor.GetComponentByClass` (`self.GetOwner`) "/Game/Main/Blueprints/PlayerComponents/Camera/BP_ViewModeComponent.BP_ViewModeComponent_C")))

(event `self.ReceiveTick`
  (params (DeltaSeconds :type "Float (single-precision)"))
  (`parent.ReceiveTick` DeltaSeconds))

(event `Test`
  (`KismetSystemLibrary.PrintString` (`KismetStringLibrary.Conv_BoolToString` (`self.CheckAvalibleDoing`)))
  (`KismetSystemLibrary.PrintString` (`KismetStringLibrary.Conv_BoolToString` (`self.isAvailable`)) true true (struct :`R` 0.395744 :`G` 1.0 :`B` 0.990052 :`A` 1.0))
  (`KismetSystemLibrary.PrintString` (`KismetStringLibrary.Conv_BoolToString` (`self.partnerIsAvalible`)) true true (struct :`R` 0.208059 :`G` 0.980103 :`B` 1.0 :`A` 1.0))
  (`self.Start`)
  (`KismetSystemLibrary.Delay` 0.2)
  (`self.Action`))

(event `self.Stop`
  (`self.StopIteraction`)
  (`self.ServerTransferStatus` (`self.status`))
  (`self.StatusChangeEventDispatcher` (`self.status`) (`self.CheckAvalibleDoing`))
  (bind _mainview (message `/Game/Main/Blueprints/MainProjectPart/BPI_HUDProject.GetMainWidget` (`PlayerController.GetHUD` (`GameplayStatics.GetPlayerController` 0))))
  (message `/Game/Main/Widgets/Reactions/BPI_ReactionView.SetShowHighfive` _mainview false)
  (bind _mainview_2 (message `/Game/Main/Blueprints/MainProjectPart/BPI_HUDProject.GetMainWidget` (`PlayerController.GetHUD` (`GameplayStatics.GetPlayerController` 0))))
  (message `/Game/Main/Widgets/Reactions/BPI_ReactionView.SetShowStopDoing` _mainview_2 false))

(event `self.Action`
  (bind _output_get (set `self.status` "NewEnumerator2"))
  (`self.StatusChangeEventDispatcher` (`self.status`) (`self.CheckAvalibleDoing`))
  (message `/Game/Main/Blueprints/PlayerComponents/Interaction/HumanoidInteraction/SceneComponent/BPI_SceneSlot.SetSlot` (`self.slotComponent`) (`self.partner`))
  (`self.ServerApplyAction` _output_get (`self.partner`))
  (`KismetSystemLibrary.Delay` 1.0)
  (`self.Stop`))

(event `self.Start`
  (`self.StartIteraction`)
  (`self.Apply Action by Status` (`self.status`))
  (`self.StatusChangeEventDispatcher` (`self.status`) (`self.CheckAvalibleDoing`))
  (`self.ServerTransferStatus` (`self.status`)))

(event `ServerApplyAction`
  (params (status :type "/Game/Main/Blueprints/PlayerComponents/Interaction/HumanoidInteraction/Emum/E_HumanoidIteractionStatus Enum" :default "NewEnumerator0") (partnerActor :type "Actor Object Reference"))
  (`self.ClientApplyActionByStatus` status partnerActor))

(event `ClientTransferStatus`
  (params (status :type "/Game/Main/Blueprints/PlayerComponents/Interaction/HumanoidInteraction/Emum/E_HumanoidIteractionStatus Enum" :default "NewEnumerator0"))
  (set `self.status` status))

(event `ServerTransferStatus`
  (params (status :type "/Game/Main/Blueprints/PlayerComponents/Interaction/HumanoidInteraction/Emum/E_HumanoidIteractionStatus Enum" :default "NewEnumerator0"))
  (bind _output_get (set `self.status` status))
  (`self.ClientTransferStatus` _output_get))

(event `ClientApplyActionByStatus`
  (params (status :type "/Game/Main/Blueprints/PlayerComponents/Interaction/HumanoidInteraction/Emum/E_HumanoidIteractionStatus Enum" :default "NewEnumerator0") (partnerActor :type "Actor Object Reference"))
  (bind _output_get (set `self.partner` partnerActor))
  (`/Engine/EditorBlueprintResources/StandardMacros.IsValid` _output_get
    (:`Is Valid`
      (`/Game/Main/Blueprints/PlayerComponents/Player/BP_ControlComponent.SetLockInputEvent` (`Actor.GetComponentByClass` (`self.partner`) "/Game/Main/Blueprints/PlayerComponents/Player/BP_ControlComponent.BP_ControlComponent_C") true)
      (`/Game/Main/Blueprints/PlayerComponents/Player/BP_ControlComponent.SetLockInputEvent` (`self.controlComponent`) true)
      (`KismetSystemLibrary.Delay` 2.0)
      (`self.Apply Action by Status` status)
      (`self.Apply Action by Status` (`Actor.GetComponentByClass` (`self.partner`) "BP_HighFiveComponent_C") status)
      (`KismetSystemLibrary.Delay` 2.0)
      (`/Game/Main/Blueprints/PlayerComponents/Player/BP_ControlComponent.SetLockInputEvent` (`self.controlComponent`) false)
      (`/Game/Main/Blueprints/PlayerComponents/Player/BP_ControlComponent.SetLockInputEvent` (`Actor.GetComponentByClass` (`self.partner`) "/Game/Main/Blueprints/PlayerComponents/Player/BP_ControlComponent.BP_ControlComponent_C") false)
      (`self.Stop`))
    (:`Is Not Valid`
      (`self.Stop`))))

(event `ServerInviteAction`
  (params (partner :type "Actor Object Reference") (isValid :type Boolean))
  (bind _returnvalue (`Actor.GetComponentByClass` partner "BP_HighFiveComponent_C"))
  (`/Engine/EditorBlueprintResources/StandardMacros.IsValid` partner
    (:`Is Valid`
      (if isValid
        (`self.SetShowDisplay` _returnvalue true)
        (message `/Game/Main/Blueprints/PlayerComponents/Interaction/HumanoidInteraction/BPI_HumanoidInteraction.SetInviteStage` _returnvalue true)
        (bind _value (message `/Game/Main/Blueprints/PlayerComponents/Interaction/HumanoidInteraction/BPI_HumanoidInteraction.GetInviteStage` _returnvalue))
        (`KismetSystemLibrary.PrintString` (`KismetStringLibrary.Concat_StrStr` "Приглашение " (`KismetStringLibrary.Conv_BoolToString` _value) "  --- "))
        (else
          (`self.SetShowDisplay` _returnvalue false)
          (message `/Game/Main/Blueprints/PlayerComponents/Interaction/HumanoidInteraction/BPI_HumanoidInteraction.SetInviteStage` _returnvalue false)
          (`KismetSystemLibrary.PrintString` (`KismetStringLibrary.Concat_StrStr` "Приглашение " (`KismetStringLibrary.Conv_BoolToString` false))))))))

(event `SetShowDisplay`
  (params (value :type Boolean))
  (`self.ClientSetShowDisplay` value))

(event `ClientSetShowDisplay`
  (params (value :type Boolean))
  (bind _returnvalue (`PlayerController.GetHUD` (`GameplayStatics.GetPlayerController` 0)))
  (if value
    (bind _mainview (message `/Game/Main/Blueprints/MainProjectPart/BPI_HUDProject.GetMainWidget` _returnvalue))
    (message `/Game/Main/Widgets/Reactions/BPI_ReactionView.SetShowHighfive` _mainview true)
    (else
      (bind _mainview_2 (message `/Game/Main/Blueprints/MainProjectPart/BPI_HUDProject.GetMainWidget` _returnvalue))
      (message `/Game/Main/Widgets/Reactions/BPI_ReactionView.SetShowHighfive` _mainview_2 false))))

(event `self.PartherHitEvent`
  (params (partner :type "Actor Object Reference"))
  ;[1 1 1] События входа персонажа в зону
  (if (`|EnumEquality` (`self.status`) "NewEnumerator1")
    (`self.ServerInviteAction` partner true)
    (message `/Game/Main/Blueprints/PlayerComponents/Interaction/HumanoidInteraction/BPI_HumanoidInteraction.SetActivePartnerAction` (`Actor.GetComponentByClass` partner "BP_HighFiveComponent_C") (`self.GetOwner`))))

(event `self.AllowAction`
  (bind _invite (`self.invite`))
  (`KismetSystemLibrary.PrintString` (`KismetStringLibrary.Conv_BoolToString` _invite))
  (if _invite
    (`self.ServerAllowAction`)))

(event `self.NoHitEvent`
  (params (partner :type "Actor Object Reference"))
  ;[1 1 1] События входа персонажа в зону
  (`self.ServerInviteAction` partner))

(event `ServerAllowAction`
  (bind _activepartner (`self.activePartner`))
  (`KismetSystemLibrary.PrintString` (`KismetStringLibrary.Concat_StrStr` "Allow Action ----" (`KismetSystemLibrary.GetDisplayName` _activepartner)) true true (struct :`R` 1.0 :`G` 0.083511 :`B` 0.976749 :`A` 1.0) 3.0)
  (set `self.invite` false)
  (`self.ClientActionEvent` (`Actor.GetComponentByClass` _activepartner "BP_HighFiveComponent_C") _activepartner))

(event `ClientActionEvent`
  (params (actor :type "Actor Object Reference"))
  (message `/Game/Main/Blueprints/PlayerComponents/Interaction/HumanoidInteraction/BPI_HumanoidInteraction.Action` (`Actor.GetComponentByClass` actor "BP_HighFiveComponent_C"))
  (`KismetSystemLibrary.PrintString` "Hello" true true (struct :`R` 1.0 :`G` 0.083511 :`B` 0.976749 :`A` 1.0) 3.0))

(event `self.SetActivePartnerAction`
  (params (actor :type "Actor Object Reference"))
  (set `self.activePartner` actor))

(fn `Apply Action by Status`
  (params (Selection :type "/Game/Main/Blueprints/PlayerComponents/Interaction/HumanoidInteraction/Emum/E_HumanoidIteractionStatus Enum" :default "NewEnumerator0"))
  (bind _output_get (set `self.status` Selection))
  (`self.SetMontageByStatus` _output_get)
  (switch `/Game/Main/Blueprints/PlayerComponents/Interaction/HumanoidInteraction/Emum/E_HumanoidIteractionStatus` (`self.status`)
    (:`NewEnumerator0`
      (`ALSBaseCharacter.SetOverlayState` (`self.As ALS Character BP`) "Default" false)
      (`ALSBaseCharacter.Replicated_PlayMontage` (`self.As ALS Character BP`) "/Game/Main/AdditionalAnimation/Skip_Montage.Skip_Montage" 1.0))
    (:`NewEnumerator1`
      (`ALSBaseCharacter.SetOverlayState` (`self.As ALS Character BP`) "Reaction" false :!label _label)
      (`ALSBaseCharacter.Replicated_PlayMontage` (`self.As ALS Character BP`) (`self.Montage`) 1.0)
      (`KismetSystemLibrary.PrintString` "ddd"))
    (:`NewEnumerator2`
      (goto _label))))

(fn `CheckAvalibleDoing`
  (returns (value :type Boolean))
  (return (`parent.CheckAvalibleDoing`)))

(fn `GetNameHumanoidInteraction`
  (returns (Name :type String))
  (return ""))

(fn `Initialize`
  (set `self.slotComponent` (`|GetArrayItem` (`Actor.GetComponentsByInterface` (`self.GetOwner`) "/Game/Main/Blueprints/PlayerComponents/Interaction/HumanoidInteraction/SceneComponent/BPI_SceneSlot.BPI_SceneSlot_C") 1))
  (`self.InitializeCharacter`)
  (set `self.controlComponent` (`Actor.GetComponentByClass` (`self.GetOwner`) "/Game/Main/Blueprints/PlayerComponents/Player/BP_ControlComponent.BP_ControlComponent_C"))
  (cast `/ALSV4_CPP/AdvancedLocomotionV4/CharacterAssets/MannequinSkeleton/ALS_AnimBP` (`SkeletalMeshComponent.GetAnimInstance` (`ALSCharacter.SkeletalMesh` (`self.As ALS Character BP`)))))

(fn `InitializeCharacter`
  (bind _asals_character_bp (cast `/ALSV4_CPP/AdvancedLocomotionV4/Blueprints/CharacterLogic/ALS_CharacterBP` (`self.GetOwner`)))
  (set `self.As ALS Character BP` _asals_character_bp))

(fn `isAvailableStage`
  (returns (value :type Boolean))
  (return (`self.isAvailable`)))

(fn `IsProcessStage`
  (returns (value :type Boolean))
  (return (`self.isProcess`)))

(fn `SetMontageByStatus`
  (params (Selection :type "/Game/Main/Blueprints/PlayerComponents/Interaction/HumanoidInteraction/Emum/E_HumanoidIteractionStatus Enum" :default "NewEnumerator0"))
  (switch `/Game/Main/Blueprints/PlayerComponents/Interaction/HumanoidInteraction/Emum/E_HumanoidIteractionStatus` Selection
    (:`NewEnumerator0`
      (set `self.Montage` "/Game/Main/AdditionalAnimation/Emotions/Emotions/v2/OK_edited_Anim_Montage.OK_edited_Anim_Montage"))
    (:`NewEnumerator1`
      (set `self.Montage` "/Game/Main/AdditionalAnimation/Reactions/HighFive/A_HighFive_Wait_Montage.A_HighFive_Wait_Montage"))
    (:`NewEnumerator2`
      (set `self.Montage` "/Game/Main/AdditionalAnimation/Reactions/HighFive/A_HighFive_Action_Montage.A_HighFive_Action_Montage"))))

(fn `StartIteraction`
  (`parent.StartIteraction`)
  (set `self.status` "NewEnumerator1")
  (set `self.isWorking` true))

(fn `StopIteraction`
  (`parent.StopIteraction`)
  (set `self.status` "NewEnumerator0")
  (set `self.isWorking` false)
  (`/Game/Main/Blueprints/PlayerComponents/Camera/BP_ViewModeComponent.ResetViewMode` (`self.viewMode`)))