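; Humanoid interaction component that lets an ALS character ask a question, playing a gesture and showing a question message on the character's widget.
; Start moves Status through Waiting to Action, applying the Reaction overlay and replicated montage, then auto-stops after a 120-second delay.
; Stop resets the overlay, plays a skip montage and hides the HUD stop-doing message.
; Server and client events pass on status and widget visibility, alongside a status-change dispatcher.
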(event `self.ReceiveBeginPlay`
  (`parent.ReceiveBeginPlay`)
  (`self.Initialize`)
  (`KismetSystemLibrary.Delay` 0.2)
  (`self.InitializeView`))

(event `self.ReceiveTick`
  (params (DeltaSeconds :type "Float (single-precision)"))
  (`parent.ReceiveTick` DeltaSeconds))

(event `self.Stop`
  (`self.StopIteraction`)
  (`self.StatusChangeEventDispatcher` (`self.status`) (`self.CheckAvalibleDoing`))
  (`self.ServerTransferStatus` (`self.status`))
  (`self.ServerSetQuestionEvent` false)
  (`self.Apply Action by Status` (`self.status`))
  (bind _mainview (message `/Game/Main/Blueprints/MainProjectPart/BPI_HUDProject.GetMainWidget` (`PlayerController.GetHUD` (`GameplayStatics.GetPlayerController` 0))))
  (message `/Game/Main/Widgets/Reactions/BPI_ReactionView.SetShowStopDoing` _mainview false))

(event `self.Action`
  (set `self.status` "NewEnumerator2")
  (`self.StatusChangeEventDispatcher` (`self.status`) (`self.CheckAvalibleDoing`))
  (`self.ServerTransferStatus` (`self.status`))
  (`KismetSystemLibrary.Delay` 120.0)
  (`self.Stop`))

(event `self.Start`
  (`self.StartIteraction`)
  (`self.Apply Action by Status` (`self.status`))
  (`self.StatusChangeEventDispatcher` (`self.status`) (`self.CheckAvalibleDoing`))
  (`self.ServerTransferStatus` (`self.status`))
  (`self.ServerSetQuestionEvent` true)
  (`self.Action`))

(event `ServerTransferStatus`
  (params (status :type "/Game/Main/Blueprints/PlayerComponents/Interaction/HumanoidInteraction/Emum/E_HumanoidIteractionStatus Enum" :default "NewEnumerator0"))
  (set `self.status` status))

(event `ServerSetQuestionEvent`
  (params (value :type Boolean))
  (`self.ClientSetQuestionEvent` value))

(event `ClientSetQuestionEvent`
  (params (value :type Boolean))
  (message `/Game/Main/Widgets/HeadWidget/BPI_HeadWidget.SetQuestion` (`self.view`) value))

(fn `Apply Action by Status`
  (params (Selection :type "/Game/Main/Blueprints/PlayerComponents/Interaction/HumanoidInteraction/Emum/E_HumanoidIteractionStatus Enum" :default "NewEnumerator0"))
  (bind _output_get (set `self.status` Selection))
  (`self.SetMontageByStatus` _output_get)
  (switch `/Game/Main/Blueprints/PlayerComponents/Interaction/HumanoidInteraction/Emum/E_HumanoidIteractionStatus` (`self.status`)
    (:`NewEnumerator0`
      (`ALSBaseCharacter.SetOverlayState` (`self.As ALS Character BP`) "Default" true)
      (`ALSBaseCharacter.Replicated_PlayMontage` (`self.As ALS Character BP`) "/Game/Main/AdditionalAnimation/Skip_Montage.Skip_Montage" 1.0))
    (:`NewEnumerator1`
      (`ALSBaseCharacter.SetOverlayState` (`self.As ALS Character BP`) "Reaction" false :!label _label)
      (`ALSBaseCharacter.Replicated_PlayMontage` (`self.As ALS Character BP`) (`self.Montage`) 1.0)
      (`KismetSystemLibrary.PrintString` "ddd"))
    (:`NewEnumerator2`
      (goto _label))))

(fn `CheckAvalibleDoing`
  (returns (value :type Boolean))
  (return (`parent.CheckAvalibleDoing`)))

(fn `GetNameHumanoidInteraction`
  (returns (Name :type String))
  (return ""))

(fn `Initialize`
  (`self.InitializeCharacter`)
  (set `self.controlComponent` (`Actor.GetComponentByClass` (`self.GetOwner`) "/Game/Main/Blueprints/PlayerComponents/Player/BP_ControlComponent.BP_ControlComponent_C"))
  (cast `/ALSV4_CPP/AdvancedLocomotionV4/CharacterAssets/MannequinSkeleton/ALS_AnimBP` (`SkeletalMeshComponent.GetAnimInstance` (`ALSCharacter.SkeletalMesh` (`self.As ALS Character BP`)))))

(fn `InitializeCharacter`
  (bind _asals_character_bp (cast `/ALSV4_CPP/AdvancedLocomotionV4/Blueprints/CharacterLogic/ALS_CharacterBP` (`self.GetOwner`)))
  (set `self.As ALS Character BP` _asals_character_bp))

(fn `InitializeView`
  (set `self.view` (`WidgetComponent.GetWidget` (`Actor.GetComponentByClass` (`self.GetOwner`) "/Script/UMG.WidgetComponent"))))

(fn `isAvailableStage`
  (returns (value :type Boolean))
  (return (`self.isAvailable`)))

(fn `IsProcessStage`
  (returns (value :type Boolean))
  (return (`self.isProcess`)))

(fn `SetMontageByStatus`
  (params (Selection :type "/Game/Main/Blueprints/PlayerComponents/Interaction/HumanoidInteraction/Emum/E_HumanoidIteractionStatus Enum" :default "NewEnumerator0"))
  (switch `/Game/Main/Blueprints/PlayerComponents/Interaction/HumanoidInteraction/Emum/E_HumanoidIteractionStatus` Selection
    (:`NewEnumerator0`
      (set `self.Montage` "/Game/Main/AdditionalAnimation/Emotions/Emotions/v2/OK_edited_Anim_Montage.OK_edited_Anim_Montage"))
    (:`NewEnumerator1`
      (set `self.Montage` "/Game/Main/AdditionalAnimation/Emotions/Emotions/v2/question_LongAction_Montage.question_LongAction_Montage"))
    (:`NewEnumerator2`
      (set `self.Montage` "/Game/Main/AdditionalAnimation/Emotions/Emotions/v2/question_LongAction_Montage.question_LongAction_Montage"))))

(fn `StartIteraction`
  (`parent.StartIteraction`)
  (set `self.status` "NewEnumerator1")
  (set `self.isWorking` true))

(fn `StopIteraction`
  (`parent.StopIteraction`)
  (set `self.status` "NewEnumerator0")
  (set `self.isWorking` false))