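; Scene slot component for humanoid interaction that holds one actor at a fixed point on its owner, identified by id and name.
; SetSlot caches the component's world transform and passes it to ServerSetSlot, which teleports the actor there.
; Both actors' BP_ControlComponents then receive rotations, with the owner's yaw offset 180 degrees from the slot's.
; The OnRep handlers are empty, and a debug box and prints remain.
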(event `self.ReceiveBeginPlay`
  (`KismetSystemLibrary.Delay` 0.2)
  (`KismetSystemLibrary.DrawDebugBox` (0.0 0.0 0.0) (0.2 0.2 0.2) (struct :`R` 1.0 :`B` 0.025978 :`A` 1.0) (struct) 5.0 1.0))

(event `/Game/Main/Blueprints/PlayerComponents/Interaction/HumanoidInteraction/SceneComponent/BPI_SceneSlot.SetSlotId`
  (params (id :type Integer))
  (set `self.id` id))

(event `/Game/Main/Blueprints/PlayerComponents/Interaction/HumanoidInteraction/SceneComponent/BPI_SceneSlot.SetSlotName`
  (params (name :type String))
  (set `self.name` name))

(event `/Game/Main/Blueprints/PlayerComponents/Interaction/HumanoidInteraction/SceneComponent/BPI_SceneSlot.SetSlot`
  (params (actor :type "Actor Object Reference"))
  (set `self.containedActor` actor)
  (`self.UpdateSlotLocationAndRotation`)
  (`self.ServerSetSlot` (`self.containedActor`) (`self.location`) (`self.rotation`)))

(event `ServerSetSlot`
  (params (containedActor :type "Actor Object Reference") (location :type "Vector Structure") (rotation :type "Rotator Structure"))
  (bind _output_get (set `self.containedActor` containedActor))
  (`/Engine/EditorBlueprintResources/StandardMacros.IsValid` _output_get
    (:`Is Valid`
      (set `self.location` location)
      (set `self.rotation` rotation)
      (`|ExecutionSequence`
        (:`then_0`
          (`Actor.K2_SetActorLocationAndRotation` (`self.containedActor`) (`self.location`) (`self.rotation`) false true))
        (:`then_1`
          (`self.SetPlayerRotation`))
        (:`then_2`
          (`KismetSystemLibrary.PrintString` "Scene slot" true true (struct :`R` 0.045979 :`G` 1.0 :`B` 0.071539 :`A` 1.0)))))))

(fn `GetSlot`
  (returns (actor :type "Actor Object Reference"))
  (return (`self.containedActor`)))

(fn `GetSlotId`
  (returns (id :type Integer))
  (return (`self.id`)))

(fn `GetSlotLocationAndRotation`
  (returns (location :type "Vector Structure") (rotation :type "Rotator Structure"))
  (`self.UpdateSlotLocationAndRotation`)
  (return (`self.location`) (`self.rotation`)))

(fn `GetSlotName`
  (returns (name :type String))
  (return (`self.name`)))

(fn `OnRep_containedActor`)

(fn `OnRep_location`)

(fn `OnRep_rotation`)

(fn `SetPlayerRotation`
  (bind _rotation (`self.rotation`))
  (`/Game/Main/Blueprints/PlayerComponents/Player/BP_ControlComponent.SetPlayerRotationEvent` (`Actor.GetComponentByClass` (`self.containedActor`) "/Game/Main/Blueprints/PlayerComponents/Player/BP_ControlComponent.BP_ControlComponent_C") _rotation)
  (`/Game/Main/Blueprints/PlayerComponents/Player/BP_ControlComponent.SetPlayerRotationEvent` (`Actor.GetComponentByClass` (`self.GetOwner`) "/Game/Main/Blueprints/PlayerComponents/Player/BP_ControlComponent.BP_ControlComponent_C") (`KismetMathLibrary.MakeRotator` (.roll _rotation) (.pitch _rotation) (- (.yaw _rotation) 180.0))))

(fn `UpdateSlotLocationAndRotation`
  (set `self.location` (`self.K2_GetComponentLocation` self))
  (bind _output_get (set `self.rotation` (`self.K2_GetComponentRotation` self)))
  (`KismetSystemLibrary.PrintString` (`KismetStringLibrary.Conv_RotatorToString` _output_get)))