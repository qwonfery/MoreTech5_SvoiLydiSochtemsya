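; Pawn component that lets the player find and use interactable objects, with a helper that traces a drop location.
; On the local autonomous proxy, a looping timer traces from the ALS camera, at view-mode-dependent range, for BPI_ObjectInteration components and toggles HUD prompts.
; Fetching actions broadcasts them and pauses the timer until the trace loses a target.
; A selected action goes through a server event to the object, and the result returns through a client event.
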(event `self.ReceiveBeginPlay`
  (`self.InitializePlayerCameraManager`)
  (bind _aspawn (cast `Pawn` (`self.GetOwner` self)))
  (set `self.subjectPawn` _aspawn)
  (`KismetSystemLibrary.Delay` 0.2)
  (bind _output_get (set `self.role` (`Actor.GetLocalRole` (`self.GetOwner`))))
  (if (`|EnumEquality` _output_get "ROLE_AutonomousProxy")
    (if (`Controller.IsLocalController` (`GameplayStatics.GetPlayerController` 0))
      (bind _returnvalue (`KismetSystemLibrary.K2_SetTimerDelegate` (delegate `InteroperabilityQualifierEvent`) 0.05 true))
      (set `self.timerEffectTickHandle` _returnvalue)
      (add `/Game/Main/Blueprints/PlayerComponents/Camera/BP_ViewModeComponent.OnChangeViewMode` (`Actor.GetComponentByClass` (`self.GetOwner`) "/Game/Main/Blueprints/PlayerComponents/Camera/BP_ViewModeComponent.BP_ViewModeComponent_C") (delegate `OnChangeViewModeEvent`))
      (set `self.hud` (`PlayerController.GetHUD` (`GameplayStatics.GetPlayerController` 0)))
      (message `/Game/Main/Blueprints/MainProjectPart/BPI_HUDProject.SetAvalibleAction` (`self.hud`) false))))

(event `InteroperabilityQualifierEvent`
  (bind (_isvalid _objectinteraction) (`self.GetObjectInteraction`))
  (`/Engine/EditorBlueprintResources/StandardMacros.IsValid` _objectinteraction
    (:`Is Valid`
      (if _isvalid
        (message `/Game/Main/Blueprints/MainProjectPart/BPI_HUDProject.SetAvalibleAction` (`self.hud`) true)
        (if (`self.autoGetAvalibleAction`)
          (`self.SubjectGetAllAvalibleActions`))))
    (:`Is Not Valid`
      (message `/Game/Main/Blueprints/MainProjectPart/BPI_HUDProject.SetAvalibleAction` (`self.hud`) false))))

(event `OnChangeViewModeEvent`
  (params (viewMode :type "/Game/Main/Blueprints/PlayerComponents/Camera/Enum/E_ViewMode Enum" :default "NewEnumerator0"))
  (switch `/Game/Main/Blueprints/PlayerComponents/Camera/Enum/E_ViewMode` viewMode
    (:`NewEnumerator0`
      (set `self.distance` 150.0))
    (:`NewEnumerator1`
      (set `self.distance` 400.0))))

(event `GetAllObjectActionEvent`
  (bind (_isvalid _objectinteraction) (`self.GetObjectInteraction`))
  (bind (_isvalid_2 _objectinteraction_2) (`self.GetObjectInteraction`))
  (bind _hud (`self.hud`))
  (if _isvalid
    (bind _output_get (set `self.objectInteraction` _objectinteraction))
    (bind (_mapidactionname _mapidname) (message `/Game/Main/Blueprints/PlayerComponents/Interaction/BPI_ObjectInteration.GetMapIdActionName` _output_get))
    ;[1 1 1] Оправка на View
    (`self.OnChangeAvalibleActions` _mapidactionname _mapidname)
    (`KismetSystemLibrary.K2_PauseTimerHandle` (`self.timerEffectTickHandle`))
    (message `/Game/Main/Blueprints/MainProjectPart/BPI_HUDProject.SetActionSelection` _hud true)
    (message `/Game/Main/Blueprints/MainProjectPart/BPI_HUDProject.SetAvalibleAction` _hud false)
    (`/Engine/EditorBlueprintResources/StandardMacros.IsValid` _objectinteraction_2
      (:`Is Valid`
        (if _isvalid_2 :!label _label
          (`KismetSystemLibrary.Delay` 1.0)
          (goto _label)
          (else
            (message `/Game/Main/Blueprints/MainProjectPart/BPI_HUDProject.SetActionSelection` (`self.hud`) false)
            (`KismetSystemLibrary.K2_UnPauseTimerHandle` (`self.timerEffectTickHandle`))))))))

(event `SelectActionEvent`
  (params (idAction :type Integer))
  (`self.ServerInteractEvent` (`self.objectInteraction`) (`self.subjectPawn`) idAction))

(event `ServerInteractEvent`
  (params (objectInteraction :type "ActorComponent Object Reference") (interactingPawn :type "Pawn Object Reference") (objectActionId :type Integer))
  (bind (_interactionstatus _actionstatus) (`self.Interact` objectInteraction interactingPawn objectActionId))
  (`self.ClientInteractResultEvent` _interactionstatus _actionstatus))

(event `ClientInteractResultEvent`
  (params (result :type "/Game/Main/Blueprints/PlayerComponents/Interaction/EInteractionStatus Enum" :default "NewEnumerator0") (`Action Status` :type "/Game/Main/Blueprints/PlayerComponents/Interaction/EActionStatus Enum" :default "NewEnumerator0"))
  (`self.OnChangeInteractResult` result))

(event `self.SubjectIteract`)

(event `self.SubjectSelectAction`
  (params (idAction :type Integer))
  (`self.SelectActionEvent` idAction))

(event `self.SubjectGetAllAvalibleActions`
  (`self.GetAllObjectActionEvent`))

(event `ShowActionMessageEvent`
  (params (value :type Boolean)))

(event `SetActionMessageEvent`
  (params (actionMessage :type Text)))

(fn `GetDropLocation`
  (returns (result :type "Vector Structure"))
  (bind _returnvalue (`Actor.GetComponentByClass` (`self.GetOwner`) "/Script/Engine.ArrowComponent"))
  (bind _returnvalue_2 (`SceneComponent.K2_GetComponentLocation` _returnvalue))
  (bind (_outhit _returnvalue_3) (`KismetSystemLibrary.LineTraceSingleForObjects` :`Start` _returnvalue_2 :`End` (+ _returnvalue_2 (* (+ (`SceneComponent.GetForwardVector` _returnvalue) (0.0 0.0 -0.9)) 100000.0)) :`ObjectTypes` (`|MakeArray` "ObjectTypeQuery4" "ObjectTypeQuery3" "ObjectTypeQuery1" "ObjectTypeQuery2" "ObjectTypeQuery5" :!type "EObjectTypeQuery Enum") :`DrawDebugType` "ForOneFrame" :`TraceColor` (struct :`R` 0.035046 :`B` 1.0 :`A` 1.0) :`DrawTime` 2.0))
  (if _returnvalue_3
    (return (`.ImpactPoint` (`GameplayStatics.BreakHitResult` _outhit)))
    (else
      (return (1.0 1.0 1.0)))))

(fn `GetObjectInteraction`
  (returns (isValid :type Boolean) (objectInteraction :type "ActorComponent Object Reference"))
  (bind _transformcomponent (`PlayerCameraManager.TransformComponent` (`self.Player Camera Manager`)))
  (bind _returnvalue (`SceneComponent.K2_GetComponentLocation` _transformcomponent))
  (bind (_outhit _returnvalue_2) (`KismetSystemLibrary.LineTraceSingle` _returnvalue (+ _returnvalue (* (`SceneComponent.GetForwardVector` _transformcomponent) (`self.distance`))) "TraceTypeQuery1"))
  (if _returnvalue_2
    (bind _output (`|GetArrayItem` (`Actor.GetComponentsByInterface` (`.HitActor` (`GameplayStatics.BreakHitResult` _outhit)) "/Game/Main/Blueprints/PlayerComponents/Interaction/BPI_ObjectInteration.BPI_ObjectInteration_C")))
    (`/Engine/EditorBlueprintResources/StandardMacros.IsValid` _output
      (:`Is Valid`
        (return true _output))
      (:`Is Not Valid`
        (return false null)))
    (else
      (return false null))))

(fn `InitializePlayerCameraManager`
  (bind _asals_player_controller (cast `/ALSV4_CPP/AdvancedLocomotionV4/Blueprints/CharacterLogic/ALS_Player_Controller` (`GameplayStatics.GetPlayerController` 0)))
  (set `self.Player Camera Manager` (`PlayerController.PlayerCameraManager` _asals_player_controller)))

(fn `Interact`
  (params (objectInteraction :type "ActorComponent Object Reference") (interactingPawn :type "Pawn Object Reference") (objectActionId :type Integer))
  (returns (interactionStatus :type "/Game/Main/Blueprints/PlayerComponents/Interaction/EInteractionStatus Enum") (actionStatus :type "/Game/Main/Blueprints/PlayerComponents/Interaction/EActionStatus Enum"))
  (bind (_interactionstatus _actionstatus) (message `/Game/Main/Blueprints/PlayerComponents/Interaction/BPI_ObjectInteration.Interact` objectInteraction objectActionId interactingPawn))
  (`|ExecutionSequence`
    (:`then_0`
      (return _interactionstatus _actionstatus))
    (:`then_1`
      (`KismetSystemLibrary.PrintString` (`KismetStringLibrary.Concat_StrStr` "Subject Interaction: " (`|GetEnumeratorNameAsString` _interactionstatus))))))

(fn `SubjectGetDropLocation`
  (returns (result :type "Vector Structure"))
  (bind _result (`self.GetDropLocation`))
  (return _result))