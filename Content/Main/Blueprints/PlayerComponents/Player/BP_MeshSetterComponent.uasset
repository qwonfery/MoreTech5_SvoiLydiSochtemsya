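; Player component that sets and syncs the owning character's skeletal mesh across the network.
; On the autonomous proxy, it reads the chosen mesh from the game instance and sends it to the server on BeginPlay.
; The server stores it and multicasts it, so each instance applies it to the owner's skeletal mesh component and calls OnChangeMesh.
; Separate events allow re-initialization, direct mesh changes and re-broadcasting the stored mesh.
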(event `self.ReceiveBeginPlay`
  (`self.InitializeMesh`)
  (if (`|EnumEquality` (`Actor.GetLocalRole` (`self.GetOwner`)) "ROLE_AutonomousProxy")
    (`self.ServerSetPlayerMesh` (`self.PlayerMesh`))))

(event `ServerApplyPlayerMesh`
  (params (mesh :type "SkeletalMesh Object Reference"))
  (bind _output_get (set `self.PlayerMesh` mesh))
  (`self.ApplyPlayerMesh` _output_get)
  (`self.ServerSetPlayerMesh` _output_get))

(event `ServerSetPlayerMesh`
  (params (PlayerMesh :type "SkeletalMesh Object Reference"))
  (bind _output_get (set `self.PlayerMesh` PlayerMesh))
  (`self.MulticastShowPlayerMesh` _output_get))

(event `MulticastShowPlayerMesh`
  (params (PlayerMesh :type "SkeletalMesh Object Reference"))
  (`self.ApplyPlayerMesh` PlayerMesh)
  (`self.OnChangeMesh`))

(event `/Game/Main/Blueprints/PlayerComponents/Player/Interface/BPI_PlayerMesh.SetPlayerMesh`
  (params (mesh :type "SkeletalMesh Object Reference"))
  (`self.MulticastShowPlayerMesh` mesh))

(event `/Game/Main/Blueprints/PlayerComponents/Player/Interface/BPI_Initializer.Initialize`
  (bind _playermesh (`self.PlayerMesh`))
  (`self.InitializeMesh`)
  (`self.ApplyPlayerMesh` _playermesh)
  (`self.ServerSetPlayerMesh` _playermesh))

(event `/Game/Main/Blueprints/MainProjectPart/Services/BPI_ServerDataRecipient.ServerUpdateData`
  (`self.MulticastShowPlayerMesh` (`self.PlayerMesh`)))

(fn `ApplyPlayerMesh`
  (params (NewMesh :type "SkeletalMesh Object Reference"))
  (`SkinnedMeshComponent.SetSkinnedAssetAndUpdate` (`Actor.GetComponentByClass` (`self.GetOwner`) "/Script/Engine.SkeletalMeshComponent") NewMesh true))

(fn `GetPlayerMesh`
  (returns (mesh :type "SkeletalMesh Object Reference"))
  (return (`self.PlayerMesh`)))

(fn `InitializeMesh`
  (if (`|EnumEquality` (`Actor.GetLocalRole` (`self.GetOwner`)) "ROLE_AutonomousProxy")
    (bind _mesh (message `/Game/Main/Blueprints/PlayerComponents/Player/Interface/BPI_PlayerMesh.GetPlayerMesh` (`GameplayStatics.GetGameInstance`)))
    (`/Engine/EditorBlueprintResources/StandardMacros.IsValid` _mesh
      (:`Is Valid`
        (set `self.PlayerMesh` _mesh))
      (:`Is Not Valid`
        (`KismetSystemLibrary.PrintString` "Не получил меш игрока из гайминстанса" true true (struct :`R` 1.0 :`B` 0.10567 :`A` 1.0))))))