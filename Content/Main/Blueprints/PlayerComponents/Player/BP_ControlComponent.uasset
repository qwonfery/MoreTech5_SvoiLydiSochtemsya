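; BP_ControlComponent is a player component for an ALS character that handles input locking, teleporting and mesh rotation.
; BeginPlay caches player controller 0, the owner, its ALS movement component and skeletal mesh.
; Server-prefixed events move and rotate character or mesh, forcing Aiming mode for full teleports and briefly activating inactive movement for location-only moves.
; Pawn rotation and lobby-opening events are stubs, and the StartRotationMesh capture is disconnected.
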(event `self.ReceiveBeginPlay`
  (set `self.playerController` (`GameplayStatics.GetPlayerController` 0))
  (set `self.movementComponent` (`Actor.GetComponentByClass` (`self.GetOwner`) "/Script/ALSV4_CPP.ALSCharacterMovementComponent"))
  (set `self.mainActor` (`self.GetOwner`))
  (set `self.baseCharacterMesh` (`Actor.GetComponentByClass` (`self.GetOwner`) "/Script/Engine.SkeletalMeshComponent")))

(event `SetLockInputEvent`
  (params (value :type Boolean))
  (bind _playercontroller (`self.playerController`))
  (if (`KismetSystemLibrary.IsValid` (`self.playerController`))
    (if value
      (`Actor.DisableInput` (`self.mainActor`) (`self.playerController`))
      (else
        (`Actor.EnableInput` _playercontroller _playercontroller)
        (`Actor.EnableInput` (`self.mainActor`) _playercontroller)))))

(event `SetPlayerControllerRotationEvent`
  (params (rotation :type "Rotator Structure"))
  (`Controller.SetControlRotation` (`self.playerController`) rotation))

(event `SetPlayerPawnRotationEvent`
  (params (rotation :type "Rotator Structure")))

(event `ServerSetLocationAndRotationEvent`
  (params (NewLocation :type "Vector Structure") (NewRotation :type "Rotator Structure") (bTeleport :type Boolean) (Target :type "Actor Object Reference"))
  (bind _returnvalue (`self.GetOwner`))
  (bind _asals_character_bp (cast `/ALSV4_CPP/AdvancedLocomotionV4/Blueprints/CharacterLogic/ALS_CharacterBP` _returnvalue))
  (`ALSBaseCharacter.SetRotationMode` _asals_character_bp "Aiming" true)
  (`ALSBaseCharacter.SetActorLocationAndTargetRotation` _asals_character_bp NewLocation NewRotation)
  (`KismetSystemLibrary.PrintString` (`KismetStringLibrary.Conv_RotatorToString` (`Actor.K2_GetActorRotation` _returnvalue)))
  (`KismetSystemLibrary.PrintString` "TP" true true (struct :`R` 1.0 :`G` 0.088576 :`A` 1.0))
  (`self.SetPlayerControllerRotationEvent` NewRotation))

(event `/Game/Main/Blueprints/PlayerComponents/Player/Interface/BPI_ControlComponent.SetLocationAndRotation`
  (params (newLocation :type "Vector Structure") (newRotation :type "Rotator Structure") (teleport :type Boolean) (target :type "Actor Object Reference"))
  (`self.ServerSetLocationAndRotationEvent` newLocation newRotation teleport target))

(event `TryOpenLobbyEvent`
  (if (`self.lobbyAvalible`)
    _))

(event `ServerRotationMeshEvent`
  (params (`X (Roll)` :type "Float (double-precision)") (`Y (Pitch)` :type "Float (double-precision)") (`Z (Yaw)` :type "Float (double-precision)"))
  (bind _output_get (set `self.New Rotatation` (`KismetMathLibrary.MakeRotator` `X (Roll)` `Y (Pitch)` `Z (Yaw)`)))
  (`SceneComponent.K2_SetWorldRotation` (`self.baseCharacterMesh`) _output_get false true))

(event `ServerBaseRelativeRotationMeshEvent`
  (`SceneComponent.K2_SetRelativeRotation` (`self.baseCharacterMesh`) (`self.startRotationMesh`) false true))

(event `ServerSetLocationEvent`
  (params (NewLocation :type "Vector Structure") (Target :type "Actor Object Reference"))
  (bind _returnvalue (`Actor.K2_GetActorRotation` (`self.Target`)))
  (set `self.New Location` NewLocation)
  (set `self.Target` Target)
  (bind _asals_character_bp (cast `/ALSV4_CPP/AdvancedLocomotionV4/Blueprints/CharacterLogic/ALS_CharacterBP` (`self.Target`)))
  (if (`self.IsActive` (`self.movementComponent`))
    (`ALSBaseCharacter.SetActorLocationAndTargetRotation` _asals_character_bp (`self.New Location`) _returnvalue)
    (else
      (`self.Activate` (`self.movementComponent`) true)
      (`ALSBaseCharacter.SetActorLocationAndTargetRotation` _asals_character_bp (`self.New Location`) _returnvalue)
      (`self.Deactivate` (`self.movementComponent`)))))