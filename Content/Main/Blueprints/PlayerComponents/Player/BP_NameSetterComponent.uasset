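; Player component that replicates a player's name and shows it on the owner's widget component.
; The autonomous proxy reads the name from the game instance and sends it to the server, while every instance caches the widget after a short delay.
; The owning client refreshes all pawns' name components through the game state's player array, on start and on name replication.
; Display events poll until the widget is valid.
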(event `self.ReceiveBeginPlay`
  (if (`|EnumEquality` (`Actor.GetLocalRole` (`self.GetOwner`)) "ROLE_AutonomousProxy") :!label _label
    (bind _name (`self.InitializePlayerName`))
    (`self.ServerSetPlayerName` _name)
    (`KismetSystemLibrary.Delay` 0.2)
    (`self.InitializeView`)
    (`KismetSystemLibrary.Delay` 2.0)
    (`self.RefreshAllPlayerName`)
    (else
      (`KismetSystemLibrary.Delay` 0.2)
      (`self.InitializeView`))))

(event `/Game/Main/Blueprints/PlayerComponents/Player/Interface/BPI_Initializer.Initialize`
  (goto _label))

(event `/Game/Main/Blueprints/PlayerComponents/Player/Interface/BPI_PlayerName.SetPlayerName`
  (params (name :type String))
  (`self.ServerSetPlayerName` name))

(event `ServerSetPlayerName`
  (params (PlayerName :type String))
  (set `self.name` PlayerName))

(event `MulticastShowPlayerName`
  (params (PlayerName :type String))
  (`/Engine/EditorBlueprintResources/StandardMacros.IsValid` (`self.view`) :!label _label_2
    (:`Is Valid`
      (`self.ShowPlayerName` PlayerName))
    (:`Is Not Valid`
      (`KismetSystemLibrary.Delay` 0.2)
      (goto _label_2))))

(event `RefreshNameEvent`
  (if (not (`KismetSystemLibrary.IsDedicatedServer`))
    (`/Engine/EditorBlueprintResources/StandardMacros.IsValid` (`self.view`) :!label _label_3
      (:`Is Valid`
        (`self.ShowPlayerName` (`self.name`)))
      (:`Is Not Valid`
        (`KismetSystemLibrary.Delay` 0.2)
        (goto _label_3)))))

(event `/Game/Main/Blueprints/MainProjectPart/Services/BPI_ServerDataRecipient.ServerUpdateData`
  (`self.RefreshAllPlayerDataEvent`))

(event `RefreshAllPlayerDataEvent`
  (`self.RefreshAllPlayerName`))

(fn `GetPlayerName`
  (returns (name :type String))
  (return (`self.name`)))

(fn `InitializePlayerName`
  (returns (name :type String))
  (bind _name (message `/Game/Main/Blueprints/PlayerComponents/Player/Interface/BPI_PlayerName.GetPlayerName` (`GameplayStatics.GetGameInstance`)))
  (return _name))

(fn `InitializeView`
  (bind _returnvalue (`Actor.GetComponentByClass` (`self.GetOwner`) "/Script/UMG.WidgetComponent"))
  (bind _returnvalue_2 (`WidgetComponent.GetWidget` _returnvalue))
  (`/Engine/EditorBlueprintResources/StandardMacros.IsValid` _returnvalue
    (:`Is Valid`
      (`/Engine/EditorBlueprintResources/StandardMacros.IsValid` _returnvalue_2
        (:`Is Valid`
          (set `self.view` _returnvalue_2))
        (:`Is Not Valid`
          (`KismetSystemLibrary.PrintString` "VIEW Не подгрузилось" true true (struct :`R` 1.0 :`G` 0.185218 :`A` 1.0) 4.0))))
    (:`Is Not Valid`
      (`KismetSystemLibrary.PrintString` "owner Не подгрузилось" true true (struct :`R` 1.0 :`G` 0.185218 :`A` 1.0) 4.0))))

(fn `OnRep_name`
  (if (`|EnumEquality` (`Actor.GetLocalRole` (`self.GetOwner`)) "ROLE_AutonomousProxy")
    (`self.OnChangeName` (`self.name`))
    (`self.RefreshAllPlayerName`)))

(fn `RefreshAllPlayerName`
  (if (`|EnumEquality` (`Actor.GetLocalRole` (`self.GetOwner`)) "ROLE_AutonomousProxy")
    (for _array_element (`GameStateBase.PlayerArray` (`GameplayStatics.GetGameState`))
      (bind _pawnprivate (`PlayerState.PawnPrivate` _array_element))
      (`/Engine/EditorBlueprintResources/StandardMacros.IsValid` _pawnprivate
        (:`Is Valid`
          (`self.RefreshNameEvent` (`Actor.GetComponentByClass` _pawnprivate "BP_NameSetterComponent_C")))))))

(fn `ShowPlayerName`
  (params (name :type String))
  (message `/Game/Main/Widgets/HeadWidget/BPI_HeadWidget.SetWidgetPlayerName` (`self.view`) name)
  (`KismetSystemLibrary.PrintString` (`KismetStringLibrary.Concat_StrStr` "Имя игрока: " name " Charater: " (`KismetStringLibrary.Conv_IntToString` (`PlayerState.PlayerId` (`Controller.PlayerState` (`GameplayStatics.GetPlayerController` 0))))) true true (struct :`R` 1.0 :`G` 0.188499 :`A` 1.0) 50.0))