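; Player component that lets an ALS character sit down in and stand up from a sitting zone, and reports whether that zone is available.
; On the owning client it toggles HUD prompts, interaction locks and movement, snaps to the zone's slot through the control component, and plays montages with a Sitting overlay.
; Server-named events pass on the zone, its busy flag and controller-desired rotation, while interfaces decouple it from zone and lock components.
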(event `self.ReceiveBeginPlay`
  (bind _asals_character_bp (cast `/ALSV4_CPP/AdvancedLocomotionV4/Blueprints/CharacterLogic/ALS_CharacterBP` (`self.GetOwner`)))
  (set `self.As ALS Character BP` _asals_character_bp)
  (set `self.viewMode` (`Actor.GetComponentByClass` (`self.GetOwner`) "/Game/Main/Blueprints/PlayerComponents/Camera/BP_ViewModeComponent.BP_ViewModeComponent_C"))
  (set `self.CharacterMovement` (`Actor.GetComponentByClass` (`self.GetOwner`) "/Script/ALSV4_CPP.ALSCharacterMovementComponent"))
  (set `self.controlComponent` (`Actor.GetComponentByClass` (`self.GetOwner`) "/Game/Main/Blueprints/PlayerComponents/Player/BP_ControlComponent.BP_ControlComponent_C"))
  (if (`|EnumEquality` (`Actor.GetLocalRole` (`self.GetOwner`)) "ROLE_AutonomousProxy")
    (set `self.isLocal` true)
    (else
      (set `self.isLocal` false))))

(event `StartSittingEvent`
  (bind _charactermovement (`self.CharacterMovement`))
  (`|ExecutionSequence`
    (:`then_0`
      (`self.ServerUseControllerDesiredRotation` true)
      (if (`self.isLocal`)
        (bind _mainview (message `/Game/Main/Blueprints/MainProjectPart/BPI_HUDProject.GetMainWidget` (`PlayerController.GetHUD` (`GameplayStatics.GetPlayerController` 0))))
        (message `/Game/Main/Widgets/MainGameplay/BPI_ShowSittingPanel.SetShowSittingUpPanel` _mainview true)
        (message `/Game/Main/Widgets/MainGameplay/BPI_ShowSittingPanel.SetShowSittingPanel` _mainview false)
        (set `self.IsSittingStage` true)
        (`/Game/Main/Blueprints/PlayerComponents/Player/BP_ControlComponent.SetLockInputEvent` (`self.controlComponent`) true)
        (`/Game/Main/Blueprints/PlayerComponents/Camera/BP_ViewModeComponent.ApplyThridPercon` (`self.viewMode`))
        (`self.OnChangeSittingStage` (`self.IsSittingStage`))
        (`self.SetLockInteraction` true)
        (`self.Activate` _charactermovement true)
        (`self.SetPlayerLocationAndRotation`)
        (`KismetSystemLibrary.Delay` 2.0)
        (`self.Deactivate` _charactermovement)
        (`ALSBaseCharacter.Replicated_PlayMontage` (`self.As ALS Character BP`) "/Game/MultiAnim_Rest/Animations/Sit/Default/StartEnd/MA_SittingDown_Montage.MA_SittingDown_Montage" 1.0)
        (`ALSBaseCharacter.SetOverlayState` (`self.As ALS Character BP`) "Sitting" false)
        (`KismetSystemLibrary.Delay` 1.0)
        (`ALSBaseCharacter.Replicated_PlayMontage` (`self.As ALS Character BP`) "/Game/MultiAnim_Rest/Animations/Sit/Default/StartEnd/MA_SittingLoop_Montage.MA_SittingLoop_Montage" 1.0)
        (`/Game/Main/Blueprints/PlayerComponents/Player/BP_ControlComponent.SetLockInputEvent` (`self.controlComponent`) false)))
    (:`then_1`
      (`self.ServerSetBusyZoneEvent` true))))

(event `StopSittingEvent`
  (`|ExecutionSequence`
    (:`then_0`
      (`self.ServerUseControllerDesiredRotation` false)
      (if (`self.isLocal`)
        (bind _mainview (message `/Game/Main/Blueprints/MainProjectPart/BPI_HUDProject.GetMainWidget` (`PlayerController.GetHUD` (`GameplayStatics.GetPlayerController` 0))))
        (message `/Game/Main/Widgets/MainGameplay/BPI_ShowSittingPanel.SetShowSittingUpPanel` _mainview false)
        (set `self.IsSittingStage` false)
        (`ALSBaseCharacter.Replicated_PlayMontage` (`self.As ALS Character BP`) "/Game/MultiAnim_Rest/Animations/Sit/Default/StartEnd/MA_SittingUp_Montage.MA_SittingUp_Montage" 1.0)
        (`ALSBaseCharacter.SetOverlayState` (`self.As ALS Character BP`) "Default" false)
        (`/Game/Main/Blueprints/PlayerComponents/Camera/BP_ViewModeComponent.ApplyThridPercon` (`self.viewMode`))
        (`self.OnChangeSittingStage` (`self.IsSittingStage`))
        (`self.Activate` (`self.CharacterMovement`) false)
        (`self.SetLockInteraction` false)))
    (:`then_1`
      (`self.ServerSetBusyZoneEvent` false))))

(event `/Game/Main/Blueprints/PlayerComponents/Sitting/BPI_SittingComponent.StartSitting`
  (`self.StartSittingEvent`))

(event `ServerSetBusyZoneEvent`
  (params (stage :type Boolean))
  (`self.SetBusySittingZone` stage))

(event `/Game/Main/Blueprints/PlayerComponents/Sitting/BPI_SittingComponent.StopSitting`
  (`self.StopSittingEvent`))

(event `/Game/Main/Blueprints/PlayerComponents/Sitting/BPI_SittingComponent.SetAvalible`
  (params (avalible :type Boolean))
  (bind _returnvalue (`GameplayStatics.GetPlayerController` 0))
  (bind _output_get (set `self.isAvalableStage` avalible))
  (`|ExecutionSequence`
    (:`then_0`
      (if (`self.isLocal`)
        (if (`Controller.IsLocalPlayerController` _returnvalue)
          (bind _mainview (message `/Game/Main/Blueprints/MainProjectPart/BPI_HUDProject.GetMainWidget` (`PlayerController.GetHUD` _returnvalue)))
          (message `/Game/Main/Widgets/MainGameplay/BPI_ShowSittingPanel.SetShowSittingPanel` _mainview (`self.isAvalableStage`)))))
    (:`then_1`
      (`KismetSystemLibrary.PrintString` (`KismetStringLibrary.Concat_StrStr` "Зона сидения " (`KismetStringLibrary.Conv_BoolToString` _output_get)) true true (struct :`R` 0.077081 :`G` 1.0 :`B` 0.180764 :`A` 1.0)))))

(event `/Game/Main/Blueprints/PlayerComponents/Sitting/BPI_SittingComponent.SetSittingZone`
  (params (sittingZone :type "Actor Object Reference"))
  (bind _output_get (set `self.sittingZone` sittingZone))
  (`self.ServerSetSittingZoneCustomEvent` _output_get))

(event `ServerSetSittingZoneCustomEvent`
  (params (sittingZone :type "Actor Object Reference"))
  (set `self.sittingZone` sittingZone))

(event `ServerUseControllerDesiredRotation`
  (params (stage :type Boolean))
  (set `CharacterMovementComponent.bUseControllerDesiredRotation` stage (`self.CharacterMovement`))
  (`self.ClientUseControllerDesiredRotation` stage))

(event `ClientUseControllerDesiredRotation`
  (params (`Use Controller Desired Rotation` :type Boolean))
  (set `CharacterMovementComponent.bUseControllerDesiredRotation` `Use Controller Desired Rotation` (`self.CharacterMovement`)))

(fn `IsAvalible`
  (returns (isAvalible :type Boolean))
  (bind _sittingzone (`self.sittingZone`))
  (bind _output (`|GetArrayItem` (`Actor.GetComponentsByInterface` _sittingzone "/Game/Main/Blueprints/ActorComponent/BPI_SittingZone.BPI_SittingZone_C")))
  (`|ExecutionSequence`
    (:`then_0`
      (if (`KismetSystemLibrary.IsValid` _sittingzone)
        (bind _isbusy (message `/Game/Main/Blueprints/ActorComponent/BPI_SittingZone.GetBusy` _output))
        (bind _stage (message `/Game/Main/Blueprints/ActorComponent/BPI_SittingZone.IsContainPlayer` _output))
        (bind _returnvalue (not _isbusy))
        (bind _returnvalue_2 (and _stage _returnvalue))
        (`KismetSystemLibrary.PrintString` (`KismetStringLibrary.Concat_StrStr` "Место свободно: " (`KismetStringLibrary.Conv_BoolToString` _returnvalue) " " "Содержит игрока: " (`KismetStringLibrary.Conv_BoolToString` _stage) " Вывод: " (`KismetStringLibrary.Conv_BoolToString` _returnvalue_2)))
        (return _returnvalue_2)))))

(fn `IsSitting`
  (returns (isSitting :type Boolean))
  (return (`self.IsSittingStage`)))

(fn `SetBusySittingZone`
  (params (stage :type Boolean))
  (bind _sittingzone (`self.sittingZone`))
  (bind _output (`|GetArrayItem` (`Actor.GetComponentsByInterface` _sittingzone "/Game/Main/Blueprints/ActorComponent/BPI_SittingZone.BPI_SittingZone_C")))
  (`/Engine/EditorBlueprintResources/StandardMacros.IsValid` _sittingzone
    (:`Is Valid`
      (`/Engine/EditorBlueprintResources/StandardMacros.IsValid` _output
        (:`Is Valid`
          (message `/Game/Main/Blueprints/ActorComponent/BPI_SittingZone.SetBusy` _output stage))))))

(fn `SetLockInteraction`
  (params (stage :type Boolean))
  (locals (localIsLock :type Boolean))
  (bind _returnvalue (`self.GetOwner`))
  (set `local.localIsLock` stage)
  (message `/Game/Main/Blueprints/PlayerComponents/Player/Interface/BPI_InteractionLoker.SetLockStage` (`GameplayStatics.GetPlayerController` 0) (`local.localIsLock`))
  (message `/Game/Main/Blueprints/PlayerComponents/Player/Interface/BPI_InteractionLoker.SetLockStage` _returnvalue (`local.localIsLock`))
  (for _array_element (`Actor.GetComponentsByInterface` _returnvalue "/Game/Main/Blueprints/PlayerComponents/Player/Interface/BPI_InteractionLoker.BPI_InteractionLoker_C")
    (message `/Game/Main/Blueprints/PlayerComponents/Player/Interface/BPI_InteractionLoker.SetLockStage` _array_element (`local.localIsLock`))))

(fn `SetPlayerLocationAndRotation`
  (bind _sittingzone (`self.sittingZone`))
  (if (`KismetSystemLibrary.IsValid` _sittingzone)
    (bind (_location _rotation) (message `/Game/Main/Blueprints/PlayerComponents/Interaction/HumanoidInteraction/SceneComponent/BPI_SceneSlot.GetSlotLocationAndRotation` (`|GetArrayItem` (`Actor.GetComponentsByInterface` _sittingzone "/Game/Main/Blueprints/PlayerComponents/Interaction/HumanoidInteraction/SceneComponent/BPI_SceneSlot.BPI_SceneSlot_C"))))
    (`/Game/Main/Blueprints/PlayerComponents/Player/BP_ControlComponent.ServerSetLocationAndRotation` (`self.controlComponent`) _location _rotation true (`self.GetOwner`))
    (`KismetSystemLibrary.PrintString` (`KismetStringLibrary.Concat_StrStr` (`KismetStringLibrary.Conv_VectorToString` _location) (`KismetStringLibrary.Conv_RotatorToString` _rotation)) true true (struct :`R` 0.988345 :`G` 0.874135 :`B` 1.0 :`A` 1.0))
    (else
      (`KismetSystemLibrary.PrintString` "sittingZone is not valid" true true (struct :`R` 1.0 :`B` 0.019485 :`A` 1.0)))))