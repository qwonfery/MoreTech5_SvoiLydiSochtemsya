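; Actor component that plays emotes such as greetings, thumbs up or down, laughing and crying on an ALS character.
; BeginPlay caches the owning ALS_CharacterBP; ApplyEmotion stores the emotion and maps it to a montage.
; It then sets the character's overlay state from that emotion and plays the montage through ReplicatedPlayMontage.
; ApplyEmotionStage forwards to ApplyEmotion, GetEmotionStage returns the stored emotion, and both OnRep handlers are empty.
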(event `self.ReceiveBeginPlay`
  (bind _asals_character_bp (cast `/ALSV4_CPP/AdvancedLocomotionV4/Blueprints/CharacterLogic/ALS_CharacterBP` (`self.GetOwner`)))
  (set `self.As ALS Character BP` _asals_character_bp))

(event `ApplyEmotion`
  (params (emotion :type "/Game/Main/Blueprints/PlayerComponents/Emotion/Enum/E_Emotion Enum" :default "NewEnumerator0"))
  (bind _output_get (set `self.Emotion` emotion))
  (`self.SetMontageAnimation` _output_get)
  (`ALSBaseCharacter.SetOverlayState` (`self.As ALS Character BP`) "Emotion" false)
  (`ALSBaseCharacter.Replicated_PlayMontage` (`self.As ALS Character BP`) (`self.Montage`) 1.0))

(event `/Game/Main/Blueprints/PlayerComponents/Emotion/BPI_Emotion.ApplyEmotionStage`
  (params (emotion :type "/Game/Main/Blueprints/PlayerComponents/Emotion/Enum/E_Emotion Enum" :default "NewEnumerator0"))
  (`self.ApplyEmotion` emotion))

(fn `GetEmotionStage`
  (returns (emotion :type "/Game/Main/Blueprints/PlayerComponents/Emotion/Enum/E_Emotion Enum"))
  (return (`self.Emotion`)))

(fn `OnRep_DispacherStage`)

(fn `OnRep_Emotion`)

(fn `SetMontageAnimation`
  (params (emotion :type "/Game/Main/Blueprints/PlayerComponents/Emotion/Enum/E_Emotion Enum" :default "NewEnumerator0"))
  (switch `/Game/Main/Blueprints/PlayerComponents/Emotion/Enum/E_Emotion` emotion
    (:`NewEnumerator0`
      (set `self.Montage` "/Game/Main/AdditionalAnimation/Emotions/Emotions/hello_Anim_Montage.hello_Anim_Montage"))
    (:`NewEnumerator1`
      (set `self.Montage` "/Game/Main/AdditionalAnimation/Emotions/Emotions/v2/BYE_edited_Anim_Montage.BYE_edited_Anim_Montage"))
    (:`NewEnumerator2`
      (set `self.Montage` "/Game/Main/AdditionalAnimation/Emotions/Emotions/thumbs_up_Anim_Montage.thumbs_up_Anim_Montage"))
    (:`NewEnumerator3`
      (set `self.Montage` "/Game/Main/AdditionalAnimation/Emotions/Emotions/thumbs_down_Anim_Montage.thumbs_down_Anim_Montage"))
    (:`NewEnumerator4`
      (set `self.Montage` "/Game/Main/AdditionalAnimation/Emotions/Emotions/v2/Laugh_edited_Anim_Montage.Laugh_edited_Anim_Montage"))
    (:`NewEnumerator5`
      (set `self.Montage` "/Game/Main/AdditionalAnimation/Emotions/Emotions/v2/Cry_edited_Anim_Montage.Cry_edited_Anim_Montage"))
    (:`NewEnumerator6`
      (set `self.Montage` "/Game/Main/AdditionalAnimation/Emotions/Emotions/v2/OK_edited_Anim_Montage.OK_edited_Anim_Montage"))))