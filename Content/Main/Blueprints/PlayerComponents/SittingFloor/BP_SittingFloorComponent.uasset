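; Player component that lets an ALS character sit on the floor and stand back up.
; Sitting requires not falling and ground under four downward traces at capsule center, front and both sides.
; Timed sequences play replicated montages, switch the overlay state, toggle CharacterMovement and briefly lock input.
; Interaction stays locked until standing, broadcast to player controller 0, owner and BPI_InteractionLoker components.
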(event `self.ReceiveBeginPlay`
  (bind _asals_character_bp (cast `/ALSV4_CPP/AdvancedLocomotionV4/Blueprints/CharacterLogic/ALS_CharacterBP` (`self.GetOwner`)))
  (set `self.As ALS Character BP` _asals_character_bp)
  (set `self.controlComponent` (`Actor.GetComponentByClass` (`self.GetOwner`) "/Game/Main/Blueprints/PlayerComponents/Player/BP_ControlComponent.BP_ControlComponent_C"))
  (set `self.CharacterMovement` (`Actor.GetComponentByClass` (`self.GetOwner`) "/Script/ALSV4_CPP.ALSCharacterMovementComponent")))

(event `/Game/Main/Blueprints/PlayerComponents/SittingFloor/BPI_SittingFloorComponent.StartSittingFloor`
  (`self.StartSittingFloorEvent`))

(event `/Game/Main/Blueprints/PlayerComponents/SittingFloor/BPI_SittingFloorComponent.StopSittingFloor`
  (`self.StopSittingFloorEvent`))

(event `StartSittingFloorEvent`
  (if (and (not (`self.bIsSittingFloor`)) (not (`NavMovementComponent.IsFalling` (`self.CharacterMovement`))) (`self.CheckCanSit`))
    (`self.SetLockInteraction` true)
    (`/Game/Main/Blueprints/PlayerComponents/Player/BP_ControlComponent.SetLockInputEvent` (`self.controlComponent`) true)
    (set `self.bIsSittingFloor` true)
    (`KismetSystemLibrary.Delay` 0.5)
    (`self.Deactivate` (`self.CharacterMovement`))
    (`ALSBaseCharacter.Replicated_PlayMontage` (`self.As ALS Character BP`) "/Game/MultiAnim_Rest/Animations/Sit/Default/Floor/MA_SittingFloorDown.MA_SittingFloorDown" 1.0)
    (`ALSBaseCharacter.SetOverlayState` (`self.As ALS Character BP`) "Sitting" false)
    (`KismetSystemLibrary.Delay` 2.0)
    (`ALSBaseCharacter.Replicated_PlayMontage` (`self.As ALS Character BP`) "/Game/MultiAnim_Rest/Animations/Sit/Default/Floor/MA_SittingFloorLoop.MA_SittingFloorLoop" 1.0)
    (`/Game/Main/Blueprints/PlayerComponents/Player/BP_ControlComponent.SetLockInputEvent` (`self.controlComponent`) false)))

(event `StopSittingFloorEvent`
  (if (`self.bIsSittingFloor`)
    (`self.SetLockInteraction` true)
    (`/Game/Main/Blueprints/PlayerComponents/Player/BP_ControlComponent.SetLockInputEvent` (`self.controlComponent`) true)
    (`ALSBaseCharacter.Replicated_PlayMontage` (`self.As ALS Character BP`) "/Game/MultiAnim_Rest/Animations/Sit/Default/Floor/MA_SittingFloorUp.MA_SittingFloorUp" 2.0)
    (`ALSBaseCharacter.SetOverlayState` (`self.As ALS Character BP`) "Default" false)
    (`KismetSystemLibrary.Delay` 1.0)
    (set `self.bIsSittingFloor` false)
    (`self.Activate` (`self.CharacterMovement`) true)
    (`/Game/Main/Blueprints/PlayerComponents/Player/BP_ControlComponent.SetLockInputEvent` (`self.controlComponent`) false)
    (`self.SetLockInteraction` false)))

(fn `CheckCanSit`
  (returns (bCanSit :type Boolean))
  (locals (Localndex :type Integer))
  (bind _as_als_character_bp (`self.As ALS Character BP`))
  (bind _returnvalue (`Actor.GetActorForwardVector` _as_als_character_bp))
  (bind _returnvalue_2 (`Actor.GetActorRightVector` _as_als_character_bp))
  (bind _returnvalue_3 (+ (`Actor.K2_GetActorLocation` _as_als_character_bp) (* (select `int` (`local.Localndex`) :`0` _returnvalue :`1` _returnvalue :`2` _returnvalue_2 :`3` _returnvalue_2) (* (`CapsuleComponent.GetScaledCapsuleRadius` (`Character.CapsuleComponent` _as_als_character_bp)) (select `int` (`local.Localndex`) :`0` 1.0 :`1` 0.0 :`2` 1.0 :`3` -1.0 :!type "Float (single-precision)")))))
  (for _index (range 4)
    (set `local.Localndex` _index)
    (bind (_outhit _returnvalue_4) (`KismetSystemLibrary.LineTraceSingle` _returnvalue_3 (- _returnvalue_3 (`KismetMathLibrary.MakeVector` 0.0 0.0 (+ (`CapsuleComponent.GetScaledCapsuleHalfHeight` (`Character.CapsuleComponent` _as_als_character_bp)) 25.0))) "TraceTypeQuery1"))
    (if (not _returnvalue_4)
      (return false)))
  (return true))

(fn `SetLockInteraction`
  (params (Lock :type Boolean))
  (bind _returnvalue (`self.GetOwner`))
  (message `/Game/Main/Blueprints/PlayerComponents/Player/Interface/BPI_InteractionLoker.SetLockStage` (`GameplayStatics.GetPlayerController` 0) (`local.Lock`))
  (message `/Game/Main/Blueprints/PlayerComponents/Player/Interface/BPI_InteractionLoker.SetLockStage` _returnvalue (`local.Lock`))
  (for _array_element (`Actor.GetComponentsByInterface` _returnvalue "/Game/Main/Blueprints/PlayerComponents/Player/Interface/BPI_InteractionLoker.BPI_InteractionLoker_C")
    (message `/Game/Main/Blueprints/PlayerComponents/Player/Interface/BPI_InteractionLoker.SetLockStage` _array_element (`local.Lock`))))