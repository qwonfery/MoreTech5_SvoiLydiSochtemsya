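; Game instance that holds player profile, character, audio and view settings, plus FTP and web connection info, across levels.
; Most profile, microphone and view setters write to a ProjectSaver save slot immediately; character settings stay in memory.
; Init calls InitializeSaveSystem, but its load-or-create logic is disconnected, so saved values are never restored here.
; Also opens levels by name and joins servers through "open" console commands with a hardcoded nickname.
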(event `self.ReceiveInit`
  (`self.InitializeSaveSystem`))

(event `/Game/Main/Blueprints/PlayerComponents/Player/Interface/BPI_PlayerName.SetPlayerName`
  (params (name :type String))
  (bind _output_get (set `self.selectedPlayerName` name))
  (set `/Game/Main/Blueprints/SaveSystem/ProjectSaver.playerNameSaved` _output_get (`self.projectSaver`))
  (`GameplayStatics.SaveGameToSlot` (`self.projectSaver`) (`self.slotNameSave`)))

(event `/Game/Main/Blueprints/PlayerComponents/Player/Interface/BPI_PlayerMesh.SetPlayerMesh`
  (params (mesh :type "SkeletalMesh Object Reference"))
  (bind _output_get (set `self.selectedPlayerMesh` mesh))
  (set `/Game/Main/Blueprints/SaveSystem/ProjectSaver.playerMeshSaved` _output_get (`self.projectSaver`))
  (`GameplayStatics.SaveGameToSlot` (`self.projectSaver`) (`self.slotNameSave`)))

(event `/Game/Main/Blueprints/PlayerComponents/Player/Interface/BPI_PlayerColor.SetPlayerColor`
  (params (color :type "Color Structure"))
  (bind _output_get (set `self.selectedPlayerColor` color))
  (set `/Game/Main/Blueprints/SaveSystem/ProjectSaver.playerColorSaved` _output_get (`self.projectSaver`))
  (`GameplayStatics.SaveGameToSlot` (`self.projectSaver`) (`self.slotNameSave`)))

(event `/Game/Main/Blueprints/PlayerComponents/Player/Interface/BPI_PlayerColor.SetNameColorId`
  (params (id :type Integer))
  (set `self.nameColorIndex` id))

(event `/Game/Main/Blueprints/MainProjectPart/BPI_Server.JoinServer`
  (params (IP :type String) (port :type String))
  (`self.JoinRemoteServer` IP port))

(event `/Game/Main/Blueprints/MainProjectPart/BPI_Server.JoinSelectedServer`
  (`self.JoinIpPortServer` (`self.stringServerIPPort`)))

(event `/Game/Main/Blueprints/MainProjectPart/BPI_Server.SetIpPort`
  (params (IpPort :type String))
  (set `self.stringServerIPPort` IpPort))

(event `/Game/Main/Blueprints/MainProjectPart/BPI_SceneLoader.LoadScene`
  (params (nameScene :type String))
  (`GameplayStatics.OpenLevel` (`KismetStringLibrary.Conv_StringToName` nameScene)))

(event `/Game/Main/Blueprints/ActorComponent/BPI_FTPServerInfo.SetFTPConnectStatus`
  (params (stage :type Boolean))
  (set `self.isFtpConnected` stage))

(event `self.SetMicrofonVolume`
  (params (multiple :type "Float (single-precision)"))
  (bind _output_get (set `self.microfonVolumeMultiple` multiple))
  (set `/Game/Main/Blueprints/SaveSystem/ProjectSaver.microfonVolume` _output_get (`self.projectSaver`))
  (`GameplayStatics.SaveGameToSlot` (`self.projectSaver`) (`self.slotNameSave`)))

(event `self.SetAudioDeviceById`
  (params (id :type String))
  (bind _output_get (set `self.idMicrofon` id))
  (bind _output_get_2 (set `/Game/Main/Blueprints/SaveSystem/ProjectSaver.idMicrofon` _output_get (`self.projectSaver`)))
  (`GameplayStatics.SaveGameToSlot` (`self.projectSaver`) (`self.slotNameSave`)))

(event `/Game/Main/Blueprints/PlayerComponents/Camera/BPI_ViewMode.SetViewMode`
  (params (viewMode :type "/Game/Main/Blueprints/PlayerComponents/Camera/Enum/E_ViewMode Enum" :default "NewEnumerator0"))
  (bind _output_get (set `self.viewMode` viewMode))
  (set `/Game/Main/Blueprints/SaveSystem/ProjectSaver.viewMode` _output_get (`self.projectSaver`))
  (`GameplayStatics.SaveGameToSlot` (`self.projectSaver`) (`self.slotNameSave`)))

(event `/Game/Denis/Customization/Components/Interface/BPI_CharacterSetting.SetCharacterSetting`
  (params (morph :type "Array of /Game/Denis/Customization/Structure/FMorph Structure (by ref)") (skeletalMesh :type "Array of /Game/Denis/Customization/Structure/FSkeletalMesh Structure (by ref)") (gender :type "/Game/Denis/Customization/Enum/Enum_CharacterGender Enum" :default "NewEnumerator0"))
  (set `self.Morph` morph)
  (set `self.Skeletal Mesh` skeletalMesh)
  (set `self.Gender` gender))

(fn `GetCharacterSetting`
  (returns (morph :type "Array of /Game/Denis/Customization/Structure/FMorph Structure") (skeletalMesh :type "Array of /Game/Denis/Customization/Structure/FSkeletalMesh Structure") (gender :type "/Game/Denis/Customization/Enum/Enum_CharacterGender Enum"))
  (return (`self.Morph`) (`self.Skeletal Mesh`) (`self.Gender`)))

(fn `GetFTPConnectStatus`
  (returns (stage :type Boolean))
  (return (`self.isFtpConnected`)))

(fn `GetFTPInfo`
  (returns (IP :type String) (Port :type Integer) (User :type String) (Password :type String) (WriteLogs :type Boolean) (UTF8 :type Boolean))
  (return (`self.FTPIP`) (`self.FTPPort`) (`self.FTPUser`) (`self.FTPPassword`) false true))

(fn `GetNameColorId`
  (returns (id :type Integer))
  (return (`self.nameColorIndex`)))

(fn `GetPlayerColor`
  (returns (color :type "Color Structure"))
  (locals (NewLocalVar_0 :type "Color Structure" :default (struct :`B` 133 :`G` 255 :`R` 151 :`A` 255)))
  (return (`self.selectedPlayerColor`)))

(fn `GetPlayerMesh`
  (returns (mesh :type "SkeletalMesh Object Reference"))
  (return (`self.selectedPlayerMesh`)))

(fn `GetPlayerName`
  (returns (name :type String))
  (return (`self.selectedPlayerName`)))

(fn `GetViewMode`
  (returns (viewMode :type "/Game/Main/Blueprints/PlayerComponents/Camera/Enum/E_ViewMode Enum"))
  (return (`self.viewMode`)))

(fn `GetWebDirectory`
  (returns (URLBase :type String))
  (return (`self.URLBase`)))

(fn `InitializeDefultParametrs`
  (set `self.selectedPlayerName` (`KismetStringLibrary.Concat_StrStr` "Аноним" (`KismetStringLibrary.Conv_IntToString` (`KismetMathLibrary.RandomIntegerInRange` 100 999))))
  (set `self.selectedPlayerMesh` "/ALSV4_CPP/AdvancedLocomotionV4/CharacterAssets/MannequinSkeleton/Meshes/AnimMan.AnimMan")
  (set `self.selectedPlayerColor` (struct)))

(fn `InitializeParametrsSaveSystem`
  (set `self.selectedPlayerName` (`/Game/Main/Blueprints/SaveSystem/ProjectSaver.playerNameSaved` (`self.projectSaver`)))
  (set `self.selectedPlayerMesh` (`/Game/Main/Blueprints/SaveSystem/ProjectSaver.playerMeshSaved` (`self.projectSaver`)))
  (set `self.selectedPlayerColor` (`/Game/Main/Blueprints/SaveSystem/ProjectSaver.playerColorSaved` (`self.projectSaver`)))
  (set `self.idMicrofon` (`/Game/Main/Blueprints/SaveSystem/ProjectSaver.idMicrofon` (`self.projectSaver`)))
  (set `self.microfonVolumeMultiple` (`/Game/Main/Blueprints/SaveSystem/ProjectSaver.microfonVolume` (`self.projectSaver`)))
  (set `self.viewMode` (`/Game/Main/Blueprints/SaveSystem/ProjectSaver.viewMode` (`self.projectSaver`))))

(fn `InitializeSaveSystem`)

(fn `JoinIpPortServer`
  (params (IPPort :type String))
  (`KismetSystemLibrary.ExecuteConsoleCommand` (`KismetStringLibrary.Concat_StrStr` "open " IPPort "?nickname=" "A") (`GameplayStatics.GetPlayerController` 0)))

(fn `JoinRemoteServer`
  (params (IP :type String) (Port :type String))
  (set `self.serverIP` IP)
  (set `self.serverPort` Port)
  (bind _output_get (set `self.stringServerIPPort` (`KismetStringLibrary.Concat_StrStr` IP ":" Port)))
  (`KismetSystemLibrary.ExecuteConsoleCommand` (`KismetStringLibrary.Concat_StrStr` "open " _output_get "?nickname=" "A") (`GameplayStatics.GetPlayerController` 0)))