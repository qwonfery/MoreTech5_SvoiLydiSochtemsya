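; HUD_LobbyName is a HUD Blueprint that shows the WBP_LobbyName widget when play begins.
; BeginPlay creates the widget for the first player controller, adds it to the viewport, makes it visible and gives it input focus.
; Helper functions toggle widget visibility and switch between Game-and-UI input with a mouse cursor and game-only input without one, falling back to player controller 0 when none is valid.
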(event `self.ReceiveBeginPlay`
  (`self.InitialzeMainWidget`)
  (`self.SetActivityWidget` true (`self.mainWiget`))
  (`self.SetUiInput` (`GameplayStatics.GetPlayerController` 0) (`self.mainWiget`) true))

(fn `InitialzeMainWidget`
  (bind _returnvalue (`|CreateWidget` "/Game/Main/Widgets/Lobby/WBP_LobbyName.WBP_LobbyName_C" (`GameplayStatics.GetPlayerController` 0)))
  (bind _output_get (set `self.mainWiget` _returnvalue))
  (`UserWidget.AddToViewport` _output_get 0))

(fn `SetActivityWidget`
  (params (value :type Boolean) (widget :type "UserWidget Object Reference"))
  (if value
    (`Widget.SetVisibility` widget "Visible")
    (else
      (`Widget.SetVisibility` widget "Collapsed"))))

(fn `SetUiInput`
  (params (PlayerController :type "PlayerController Object Reference") (InWidgetToFocus :type "Widget Object Reference") (value :type Boolean))
  (locals (localPlayerController :type "PlayerController Object Reference"))
  (bind _localplayercontroller (`local.localPlayerController`))
  (if (`KismetSystemLibrary.IsValid` PlayerController)
    (set `local.localPlayerController` PlayerController)
    (else
      (set `local.localPlayerController` (`GameplayStatics.GetPlayerController` 0))))
  (if value
    (`WidgetBlueprintLibrary.SetInputMode_GameAndUIEx` _localplayercontroller InWidgetToFocus "LockOnCapture")
    (set `PlayerController.bShowMouseCursor` true (`local.localPlayerController`))
    (else
      (`WidgetBlueprintLibrary.SetInputMode_GameOnly` _localplayercontroller)
      (set `PlayerController.bShowMouseCursor` false (`local.localPlayerController`)))))

(fn `UserConstructionScript`)