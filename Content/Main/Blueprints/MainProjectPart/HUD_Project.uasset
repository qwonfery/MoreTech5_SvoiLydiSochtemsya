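; Project HUD that creates and manages the player's UI widgets: action selection, emotions, reactions, bottom bar, gameplay settings, exit menu, input hint and quiz.
; BeginPlay adds every widget to the viewport and to a shared array, which also relays microphone status to all widgets.
; Events toggle widget visibility, mostly switching mouse cursor and input mode between game-only and game-and-UI.
; Admin panel, player stats and text chat getter are empty stubs.
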(event `self.ReceiveBeginPlay`
  (`self.InitialzeActionSelection`)
  (`self.InitialzeEmotion`)
  (`self.InitialzeMainDownWidget`)
  (`self.InitialzeReaction`)
  (`self.InitialzeGamePlaySitting`)
  (`self.InitialzeExitMenu`)
  (`self.InitializeInputHint`)
  (`self.InitializeQuiz`))

(event `/Game/Main/Blueprints/MainProjectPart/BPI_HUDProject.SetActiveEmotion`
  (params (value :type Boolean))
  (`self.CloseTabs`)
  (`self.SetUiInput` (`GameplayStatics.GetPlayerController` 0) value)
  (`self.SetShowStageWidget` value (`self.emotion`)))

(event `/Game/Main/Blueprints/MainProjectPart/BPI_HUDProject.SetActiveReaction`
  (params (value :type Boolean))
  (`self.CloseTabs`)
  (`self.SetUiInput` (`GameplayStatics.GetPlayerController` 0) value)
  (`self.SetShowStageWidget` value (`self.reactions`)))

(event `CloseTabs`
  (`self.SetShowStageWidget` false (`self.reactions`))
  (`self.SetShowStageWidget` false (`self.emotion`)))

(event `/Game/Main/Blueprints/MainProjectPart/BPI_HUDProject.SetGamePlaySittings`
  (params (value :type Boolean))
  (`self.SetShowStageWidget` value (`self.gamePlaySitting`))
  (`self.SetUiInput` (`GameplayStatics.GetPlayerController` 0) value))

(event `/Game/Main/Blueprints/MainProjectPart/BPI_HUDProject.SetShowExitMenu`
  (params (value :type Boolean))
  (`self.SetShowStageWidget` value (`self.ExitMenu`))
  (`self.SetUiInput` (`GameplayStatics.GetPlayerController` 0) value))

(event `/Game/Main/Blueprints/MainProjectPart/BPI_HUDProject.SetShowAdminPanel`
  (params (value :type Boolean)))

(event `/Game/Main/Widgets/MainGameplay/BPI_ShowMicStatus.SetMicrophoneWorking`
  (params (stage :type Boolean))
  (for _array_element (`self.allWidget`)
    (message `/Game/Main/Widgets/MainGameplay/BPI_ShowMicStatus.SetMicrophoneWorking` _array_element stage)))

(event `/Game/Main/Blueprints/MainProjectPart/BPI_HUDProject.SetMouseActivity`
  (params (stage :type Boolean))
  (bind _output_get (set `self.mouseActivity` stage))
  (`self.SetUiInput` (`GameplayStatics.GetPlayerController` 0) _output_get))

(event `/Game/Main/Blueprints/MainProjectPart/BPI_HUDProject.SetActionSelection`
  (params (value :type Boolean))
  (`/Game/Main/Widgets/ActionSelection/WBP_ActionSelection.ShowActionSelectionList` (`self.actionSelection`) value)
  (`self.SetUiInput` (`GameplayStatics.GetPlayerController` 0) value))

(event `/Game/Main/Blueprints/MainProjectPart/BPI_HUDProject.SetAvalibleAction`
  (params (value :type Boolean))
  (`/Game/Main/Widgets/ActionSelection/WBP_ActionSelection.ShowAvalibleAction` (`self.actionSelection`) value))

(event `/Game/Main/Blueprints/MainProjectPart/BPI_HUDProject.SetPlayerStats`
  (params (value :type Boolean)))

(event `/Game/Main/Blueprints/MainProjectPart/BPI_HUDProject.SetCursorAction`
  (params (value :type Boolean))
  (message `/Game/Main/Widgets/ActionSelection/BPI_ActionSelection.ShowCursorAction` (`self.actionSelection`) value))

(event `/Game/Main/Blueprints/MainProjectPart/BPI_HUDProject.ShowWidgetСontrolPromptEvent`
  (`/Game/Main/Widgets/InputHint/BPI_InputHint.ShowWidgetDuration` (`self.inputHint`) 5.0))

(event `/Game/Main/Blueprints/MainProjectPart/BPI_HUDProject.ShowInputHint`
  (params (value :type Boolean))
  (if (not (and value (`Widget.IsVisible` (`self.inputHint`))))
    (`self.SetShowStageWidget` value (`self.inputHint`))
    (`self.SetUiInput` null value)))

(event `/Game/Main/Blueprints/MainProjectPart/BPI_HUDProject.ShowQuiz`
  (params (value :type Boolean))
  (bind _quiz (`self.quiz`))
  (if (not (and value (`Widget.IsVisible` _quiz)))
    (`self.SetShowStageWidget` value _quiz)
    (`self.SetUiInput` null value)
    (`KismetSystemLibrary.PrintString` "Hello")))

(fn `GetAllWidget`
  (returns (widget :type "Array of UserWidget Object Reference"))
  (return (`self.allWidget`)))

(fn `GetMainWidget`
  (returns (mainView :type "UserWidget Object Reference"))
  (return (`self.mainWidget`)))

(fn `GetReactionWidget`
  (returns (reactionView :type "UserWidget Object Reference"))
  (return (`self.reactions`)))

(fn `GetTextChatWidget`
  (returns (textChatWidget :type "UserWidget Object Reference"))
  (return null))

(fn `InitializeInputHint`
  (bind _returnvalue (`|CreateWidget` "/Game/Main/Widgets/InputHint/WBP_InputHint.WBP_InputHint_C" (`GameplayStatics.GetPlayerController` 0)))
  (bind _output_get (set `self.inputHint` _returnvalue))
  (`KismetArrayLibrary.Array_Add` (`self.allWidget`) _output_get)
  (`UserWidget.AddToViewport` _output_get 0)
  (`Widget.SetVisibility` _output_get "Collapsed"))

(fn `InitializeQuiz`
  (bind _returnvalue (`|CreateWidget` "/Game/Main/Widgets/Quiz/WBP_Quiz.WBP_Quiz_C" (`GameplayStatics.GetPlayerController` 0)))
  (bind _output_get (set `self.quiz` _returnvalue))
  (`KismetArrayLibrary.Array_Add` (`self.allWidget`) _output_get)
  (`UserWidget.AddToViewport` _returnvalue 0)
  (`Widget.SetVisibility` _returnvalue "Collapsed"))

(fn `InitialzeActionSelection`
  (bind _returnvalue (`|CreateWidget` "/Game/Main/Widgets/ActionSelection/WBP_ActionSelection.WBP_ActionSelection_C" (`GameplayStatics.GetPlayerController` 0)))
  (set `self.actionSelection` _returnvalue)
  (`KismetArrayLibrary.Array_Add` (`self.allWidget`) _returnvalue)
  (`UserWidget.AddToViewport` _returnvalue 0))

(fn `InitialzeEmotion`
  (bind _returnvalue (`|CreateWidget` "/Game/Main/Widgets/Emotions/WBP_Emotions.WBP_Emotions_C" (`GameplayStatics.GetPlayerController` 0)))
  (bind _output_get (set `self.emotion` _returnvalue))
  (`KismetArrayLibrary.Array_Add` (`self.allWidget`) _output_get)
  (`UserWidget.AddToViewport` _output_get 0)
  (`Widget.SetVisibility` _output_get "Collapsed"))

(fn `InitialzeExitMenu`
  (bind _returnvalue (`|CreateWidget` "/Game/Main/Widgets/MainGameplay/WBP_ExitMenu.WBP_ExitMenu_C" (`GameplayStatics.GetPlayerController` 0)))
  (bind _output_get (set `self.ExitMenu` _returnvalue))
  (`KismetArrayLibrary.Array_Add` (`self.allWidget`) _output_get)
  (`UserWidget.AddToViewport` _output_get 0)
  (`Widget.SetVisibility` _output_get "Collapsed"))

(fn `InitialzeGamePlaySitting`
  (bind _returnvalue (`|CreateWidget` "/Game/Main/Widgets/PlayerSitting/WBP_GamePlaySitting.WBP_GamePlaySitting_C" (`GameplayStatics.GetPlayerController` 0)))
  (bind _output_get (set `self.gamePlaySitting` _returnvalue))
  (`KismetArrayLibrary.Array_Add` (`self.allWidget`) _output_get)
  (`UserWidget.AddToViewport` _output_get 0)
  (`Widget.SetVisibility` _output_get "Collapsed"))

(fn `InitialzeMainDownWidget`
  (bind _returnvalue (`|CreateWidget` "/Game/Main/Widgets/MainGameplay/WBP_MainDownWidget.WBP_MainDownWidget_C" (`GameplayStatics.GetPlayerController` 0)))
  (set `self.mainWidget` _returnvalue)
  (`KismetArrayLibrary.Array_Add` (`self.allWidget`) _returnvalue)
  (`UserWidget.AddToViewport` _returnvalue 0))

(fn `InitialzeReaction`
  (bind _returnvalue (`|CreateWidget` "/Game/Main/Widgets/Reactions/WBP_Reactions.WBP_Reactions_C" (`GameplayStatics.GetPlayerController` 0)))
  (bind _output_get (set `self.reactions` _returnvalue))
  (`KismetArrayLibrary.Array_Add` (`self.allWidget`) _output_get)
  (`UserWidget.AddToViewport` _output_get 0)
  (`Widget.SetVisibility` _output_get "Collapsed"))

(fn `SetShowStageWidget`
  (params (value :type Boolean) (widget :type "UserWidget Object Reference"))
  (if value
    (`Widget.SetVisibility` widget "Visible")
    (`KismetSystemLibrary.PrintString` "visible")
    (else
      (`Widget.SetVisibility` widget "Collapsed")
      (`KismetSystemLibrary.PrintString` "not visible"))))

(fn `SetUiInput`
  (params (PlayerController :type "PlayerController Object Reference") (value :type Boolean))
  (locals (localPlayerController :type "PlayerController Object Reference"))
  (if (`KismetSystemLibrary.IsValid` PlayerController)
    (set `local.localPlayerController` PlayerController)
    (else
      (set `local.localPlayerController` (`GameplayStatics.GetPlayerController` 0))))
  (if value
    (`WidgetBlueprintLibrary.SetInputMode_GameAndUIEx` (`GameplayStatics.GetPlayerController` 0) null "DoNotLock" false)
    (set `PlayerController.bShowMouseCursor` true (`local.localPlayerController`))
    (else
      (`WidgetBlueprintLibrary.SetInputMode_GameOnly` (`GameplayStatics.GetPlayerController` 0))
      (set `PlayerController.bShowMouseCursor` false (`local.localPlayerController`)))))

(fn `UserConstructionScript`)