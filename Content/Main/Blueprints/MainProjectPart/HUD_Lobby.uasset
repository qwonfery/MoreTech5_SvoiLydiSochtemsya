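; Lobby HUD that owns the server select, character settings and developer server select screens.
; On BeginPlay it creates all three widgets in the viewport, shows only server select and switches to Game and UI input with a visible cursor.
; Custom events toggle the settings and developer join widgets between Visible and Collapsed, and switch the player between Game and UI and Game Only input.
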(event `self.ReceiveBeginPlay`
  (`self.InitialzeMainWget`)
  (`self.SetActivityWidget` true (`self.mainWiget`))
  (`self.SetUiInput` (`GameplayStatics.GetPlayerController` 0) (`self.mainWiget`) true)
  (`self.InitialzePlayerSettings`)
  (`self.SetActivityWidget` false (`self.playerSetting`))
  (`self.InitialzeJoinCurrentServerView`)
  (`self.SetActivityWidget` false (`self.joinCurrentSeverView`)))

(event `/Game/Main/Blueprints/MainProjectPart/BPI_HUDLobby.SetShowPlayerSettingEvent`
  (params (value :type Boolean))
  (`self.SetActivityWidget` value (`self.playerSetting`)))

(event `/Game/Main/Blueprints/MainProjectPart/BPI_HUDLobby.SetShowJoinCurrentServerEvent`
  (params (value :type Boolean))
  (`self.SetActivityWidget` value (`self.joinCurrentSeverView`)))

(event `/Game/Main/Blueprints/MainProjectPart/BPI_HUDLobby.SetPlayerUiInput`
  (params (value :type Boolean))
  (`self.SetUiInput` (`GameplayStatics.GetPlayerController` 0) null value))

(fn `InitialzeJoinCurrentServerView`
  (bind _returnvalue (`|CreateWidget` "/Game/Main/Widgets/ServerSelect/WBP_ServerDeveloperSelect.WBP_ServerDeveloperSelect_C" (`GameplayStatics.GetPlayerController` 0)))
  (bind _output_get (set `self.joinCurrentSeverView` _returnvalue))
  (`UserWidget.AddToViewport` _output_get 0))

(fn `InitialzeMainWget`
  (bind _returnvalue (`|CreateWidget` "/Game/Main/Widgets/ServerSelect/WBP_ServerSelect.WBP_ServerSelect_C" (`GameplayStatics.GetPlayerController` 0)))
  (bind _output_get (set `self.mainWiget` _returnvalue))
  (`UserWidget.AddToViewport` _output_get 0))

(fn `InitialzePlayerSettings`
  (bind _returnvalue (`|CreateWidget` "/Game/Main/Widgets/PlayerSitting/WBP_CharacterSettings.WBP_CharacterSettings_C" (`GameplayStatics.GetPlayerController` 0)))
  (bind _output_get (set `self.playerSetting` _returnvalue))
  (`UserWidget.AddToViewport` _output_get 0))

(fn `SetActivityWidget`
  (params (value :type Boolean) (widget :type "UserWidget Object Reference"))
  (if value
    (`Widget.SetVisibility` widget "Visible")
    (else
      (`Widget.SetVisibility` widget "Collapsed"))))

(fn `SetUiInput`
  (params (PlayerController :type "PlayerController Object Reference") (InWidgetToFocus :type "Widget Object Reference") (value :type Boolean))
  (locals (localPlayerController :type "PlayerController Object Reference"))
  (bind _localplayercontroller (`local.localPlayerController`))
  (if (`KismetSystemLibrary.IsValid` PlayerController)
    (set `local.localPlayerController` PlayerController)
    (else
      (set `local.localPlayerController` (`GameplayStatics.GetPlayerController` 0))))
  (if value
    (`WidgetBlueprintLibrary.SetInputMode_GameAndUIEx` _localplayercontroller InWidgetToFocus "LockOnCapture")
    (set `PlayerController.bShowMouseCursor` true (`local.localPlayerController`))
    (else
      (`WidgetBlueprintLibrary.SetInputMode_GameOnly` _localplayercontroller)
      (set `PlayerController.bShowMouseCursor` false (`local.localPlayerController`)))))

(fn `UserConstructionScript`)