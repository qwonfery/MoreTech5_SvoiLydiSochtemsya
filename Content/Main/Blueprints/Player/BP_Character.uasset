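; Player character Blueprint that routes input to components for emotions, view mode, interactions and sitting.
; Number keys apply emotions; a toggle switches first and third person, and G toggles floor sitting.
; Interact runs a sequence over humanoid interaction interface components, seat, subject actions, broadcast and lobby event, while cancel stops interactions and sitting.
; A lock flag gates emotions and humanoid interactions; Q toggles HUD player stats.
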(event `self.ReceiveBeginPlay`
  (set `self.ControllerPC` (`self.GetController`))
  (set `self.widgetInteraction` (`self.GetComponentByClass` (`PlayerController.PlayerCameraManager` (`GameplayStatics.GetPlayerController` 0)) "/Script/UMG.WidgetInteractionComponent")))

(event `Key|N`
  (params (Key :type "Key Structure")))

(event `InputAction|MouseLeft`
  (params (Key :type "Key Structure")))

(event `Key|One`
  (params (Key :type "Key Structure"))
  ;[1 1 1] Горячие клавиши эмоции
  (:`Pressed`
    (if (not (`self.interactionIsLock`))
      (`/Game/Main/Blueprints/PlayerComponents/Emotion/BP_EmotionComponent.ApplyEmotion` (`self.BP_EmotionComponent`) "NewEnumerator0"))))

(event `Key|Two`
  (params (Key :type "Key Structure"))
  ;[1 1 1] Горячие клавиши эмоции
  (:`Pressed`
    (if (not (`self.interactionIsLock`))
      (`/Game/Main/Blueprints/PlayerComponents/Emotion/BP_EmotionComponent.ApplyEmotion` (`self.BP_EmotionComponent`) "NewEnumerator1"))))

(event `Key|Three`
  (params (Key :type "Key Structure"))
  ;[1 1 1] Горячие клавиши эмоции
  (:`Pressed`
    (if (not (`self.interactionIsLock`))
      (`/Game/Main/Blueprints/PlayerComponents/Emotion/BP_EmotionComponent.ApplyEmotion` (`self.BP_EmotionComponent`) "NewEnumerator2"))))

(event `Key|Four`
  (params (Key :type "Key Structure"))
  ;[1 1 1] Горячие клавиши эмоции
  (:`Pressed`
    (if (not (`self.interactionIsLock`))
      (`/Game/Main/Blueprints/PlayerComponents/Emotion/BP_EmotionComponent.ApplyEmotion` (`self.BP_EmotionComponent`) "NewEnumerator3"))))

(event `Key|Five`
  (params (Key :type "Key Structure"))
  ;[1 1 1] Горячие клавиши эмоции
  (:`Pressed`
    (if (not (`self.interactionIsLock`))
      (`/Game/Main/Blueprints/PlayerComponents/Emotion/BP_EmotionComponent.ApplyEmotion` (`self.BP_EmotionComponent`) "NewEnumerator5"))))

(event `Key|Six`
  (params (Key :type "Key Structure"))
  ;[1 1 1] Горячие клавиши эмоции
  (:`Pressed`
    (if (not (`self.interactionIsLock`))
      (`/Game/Main/Blueprints/PlayerComponents/Emotion/BP_EmotionComponent.ApplyEmotion` (`self.BP_EmotionComponent`) "NewEnumerator6"))))

(event `Key|Q`
  (params (Key :type "Key Structure"))
  (:`Pressed`
    (bind _isa (`/Engine/EditorBlueprintResources/StandardMacros.FlipFlop`)
      (:`A`
        _)
      (:`B`
        _))
    (message `/Game/Main/Blueprints/MainProjectPart/BPI_HUDProject.SetPlayerStats` (`PlayerController.GetHUD` (`GameplayStatics.GetPlayerController` 0)) _isa)
    (`KismetSystemLibrary.PrintString` "Hello")))

(event `InputAction|ViewModePlayer`
  (params (Key :type "Key Structure"))
  (:`Pressed`
    (`/Engine/EditorBlueprintResources/StandardMacros.FlipFlop`
      (:`A`
        (`/Game/Main/Blueprints/PlayerComponents/Camera/BP_ViewModeComponent.ApplyFirstPerson` (`self.BP_ViewModeComponent`)))
      (:`B`
        (`/Game/Main/Blueprints/PlayerComponents/Camera/BP_ViewModeComponent.ApplyThridPercon` (`self.BP_ViewModeComponent`))))))

(event `/Game/Main/Blueprints/PlayerComponents/Player/Interface/BPI_InteractionLoker.SetLockStage`
  (params (isLock :type Boolean))
  (bind _output_get (set `self.interactionIsLock` isLock))
  (`self.OnChangeLockStage` _output_get))

(event `InputAction|Interaction`
  (params (Key :type "Key Structure"))
  (bind _bp_sittingcomponent (`self.BP_SittingComponent`))
  ;[1 1 1] Взаимодействия
  (:`Pressed`
    (`KismetSystemLibrary.PrintString` "F")
    (`|ExecutionSequence`
      (:`then_0`
        (if (not (`self.interactionIsLock`))
          (for _array_element (`self.GetComponentsByInterface` "/Game/Main/Blueprints/PlayerComponents/Interaction/HumanoidInteraction/BPI_HumanoidInteraction.BPI_HumanoidInteraction_C")
            (bind _value (message `/Game/Main/Blueprints/PlayerComponents/Interaction/HumanoidInteraction/BPI_HumanoidInteraction.GetInviteStage` _array_element))
            (set `self.interacitionActionAvalible` _value)
            (if _value
              (message `/Game/Main/Blueprints/PlayerComponents/Interaction/HumanoidInteraction/BPI_HumanoidInteraction.AllowAction` _array_element)))))
      (:`then_1`
        (if (not (`self.interacitionActionAvalible`))
          (bind _isavalible (`/Game/Main/Blueprints/PlayerComponents/Sitting/BP_SittingComponent.IsAvalible` _bp_sittingcomponent))
          (if _isavalible
            (`/Game/Main/Blueprints/PlayerComponents/Sitting/BP_SittingComponent.StartSitting` _bp_sittingcomponent))))
      (:`then_2`
        (`/Game/Main/Blueprints/PlayerComponents/Interaction/BP_SubjectInteractionComponent.SubjectGetAllAvalibleActions` (`self.BP_SubjectInteractionComponent`)))
      (:`then_3`
        (`self.OnInteraction`))
      (:`then_4`
        (`/Game/Main/Blueprints/PlayerComponents/Player/BP_ControlComponent.TryOpenLobbyEvent` (`self.BP_ControlComponent`))))))

(event `InputAction|CancelInteraction`
  (params (Key :type "Key Structure"))
  (bind _bp_sittingcomponent (`self.BP_SittingComponent`))
  ;[1 1 1] Взаимодействия
  (:`Pressed`
    (`|ExecutionSequence`
      (:`then_0`
        (for _array_element (`self.GetComponentsByInterface` "/Game/Main/Blueprints/PlayerComponents/Interaction/HumanoidInteraction/BPI_HumanoidInteraction.BPI_HumanoidInteraction_C")
          (message `/Game/Main/Blueprints/PlayerComponents/Interaction/HumanoidInteraction/BPI_HumanoidInteraction.Stop` _array_element)))
      (:`then_1`
        (bind _issitting (`/Game/Main/Blueprints/PlayerComponents/Sitting/BPI_SittingComponent.IsSitting` _bp_sittingcomponent))
        (if _issitting
          (`/Game/Main/Blueprints/PlayerComponents/Sitting/BP_SittingComponent.StopSitting` _bp_sittingcomponent))))))

(event `Key|G`
  (params (Key :type "Key Structure"))
  (bind _bp_sittingfloorcomponent (`self.BP_SittingFloorComponent`))
  ;[1 1 1] Взаимодействия
  (:`Pressed`
    (`/Engine/EditorBlueprintResources/StandardMacros.FlipFlop`
      (:`A`
        (message `/Game/Main/Blueprints/PlayerComponents/SittingFloor/BPI_SittingFloorComponent.StartSittingFloor` _bp_sittingfloorcomponent)
        (set `self.interacitionActionAvalible` false))
      (:`B`
        (message `/Game/Main/Blueprints/PlayerComponents/SittingFloor/BPI_SittingFloorComponent.StopSittingFloor` _bp_sittingfloorcomponent)
        (set `self.interacitionActionAvalible` true)))))

(event `Key|P`
  (params (Key :type "Key Structure"))
  ;[1 1 1] Взаимодействия
)

(event `Key|LeftBracket`
  (params (Key :type "Key Structure"))
  ;[1 1 1] Взаимодействия
)

(event `Key|RightBracket`
  (params (Key :type "Key Structure"))
  ;[1 1 1] Взаимодействия
)

(fn `UserConstructionScript`
  (`parent.UserConstructionScript`))