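; BP_SittingZoneComponent is an actor component that marks its owner as a sitting zone and tracks whether it is busy or overlapped.
; It binds to the owner's box trigger and, through BPI_SittingComponent on the entering actor, signals availability and passes the owner if free.
; Leaving the trigger withdraws availability.
; The busy flag is set by event, exposed by a getter, and has a RepNotify that prints debug text.
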(event `self.ReceiveBeginPlay`
  (set `self.slotComponent` (`|GetArrayItem` (`Actor.GetComponentsByInterface` (`self.GetOwner`) "/Game/Main/Blueprints/PlayerComponents/Interaction/HumanoidInteraction/SceneComponent/BPI_SceneSlot.BPI_SceneSlot_C")))
  (set `self.triggerComponent` (`Actor.GetComponentByClass` (`self.GetOwner`) "/Script/Engine.BoxComponent"))
  (add `PrimitiveComponent.OnComponentBeginOverlap` (`self.triggerComponent`) (delegate `BeginOverlapEvent`))
  (add `PrimitiveComponent.OnComponentEndOverlap` (`self.triggerComponent`) (delegate `EndOverlapEvent`)))

(event `BeginOverlapEvent`
  (params (OverlappedComponent :type "PrimitiveComponent Object Reference") (OtherActor :type "Actor Object Reference") (OtherComp :type "PrimitiveComponent Object Reference") (OtherBodyIndex :type Integer) (bFromSweep :type Boolean) (SweepResult :type "HitResult Structure (by ref)"))
  (bind _output (`|GetArrayItem` (`Actor.GetComponentsByInterface` OtherActor "/Game/Main/Blueprints/PlayerComponents/Sitting/BPI_SittingComponent.BPI_SittingComponent_C")))
  (set `self.IsContain` true)
  (if (not (`self.isBusy`))
    (message `/Game/Main/Blueprints/PlayerComponents/Sitting/BPI_SittingComponent.SetAvalible` _output true)
    (message `/Game/Main/Blueprints/PlayerComponents/Sitting/BPI_SittingComponent.SetSittingZone` _output (`self.GetOwner`))
    (`KismetSystemLibrary.PrintString` (`KismetStringLibrary.Concat_StrStr` "Зона бегин оверлап бизи " (`KismetStringLibrary.Conv_BoolToString` (`self.isBusy`))))))

(event `EndOverlapEvent`
  (params (OverlappedComponent :type "PrimitiveComponent Object Reference") (OtherActor :type "Actor Object Reference") (OtherComp :type "PrimitiveComponent Object Reference") (OtherBodyIndex :type Integer))
  (set `self.IsContain` false)
  (message `/Game/Main/Blueprints/PlayerComponents/Sitting/BPI_SittingComponent.SetAvalible` (`|GetArrayItem` (`Actor.GetComponentsByInterface` OtherActor "/Game/Main/Blueprints/PlayerComponents/Sitting/BPI_SittingComponent.BPI_SittingComponent_C")) false))

(event `/Game/Main/Blueprints/ActorComponent/BPI_SittingZone.SetBusy`
  (params (stage :type Boolean))
  (set `self.isBusy` stage))

(fn `GetBusy`
  (returns (isBusy :type Boolean))
  (return (`self.isBusy`)))

(fn `IsContainPlayer`
  (returns (stage :type Boolean))
  (return (`self.IsContain`)))

(fn `OnRep_isBusy`
  (`KismetSystemLibrary.PrintString` (`KismetStringLibrary.Concat_StrStr` "SittingZone Busy " (`KismetStringLibrary.Conv_BoolToString` (`self.isBusy`))) true true (struct :`R` 1.0 :`G` 0.322369 :`B` 0.312421 :`A` 1.0)))